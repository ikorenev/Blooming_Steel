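; Behavior tree task that picks the next patrol destination for a BP_Enemy_AI pawn.
; It reads the LCPI index from the blackboard, resets it to zero when out of range, and writes that PP actor's location to the Key blackboard entry.
; It then stores the incremented index, so successive runs loop through the points.
; It finishes successfully even with no points, but never finishes if the cast fails.
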(event EventReceiveExecuteAI
  (params (OwnerController :type AI%20Controller%20Object%20Reference) (ControlledPawn :type Pawn%20Object%20Reference))
  (bind _returnvalue (Utilities|Name|MakeLiteralName "LCPI"))
  (bind _blackboardkeyselector (Utilities|Struct|MakeBlackboardKeySelector _returnvalue))
  (bind _returnvalue_2 (Class|BTFunctionLibrary|GetBlackboardValueasInt _blackboardkeyselector))
  (bind _asbp_enemy_ai (Utilities|Casting|CastToBP_Enemy_AI ControlledPawn))
  (bind _output_get (Variables|Default|SetP%20P (Variables|/Game/AssetCore/Blueprints/AI/BP_Enemy_AI.BP_Enemy_AI_C|GetP_P _asbp_enemy_ai)))
  (if (> (Utilities|Array|Length _output_get) 0)
    (if (Utilities|Array|IsValidIndex (Variables|Default|GetP%20P) _returnvalue_2)
      (Variables|Default|SetLCPI _returnvalue_2)
      (else
        (Variables|Default|SetLCPI 0)))
    (AI|BehaviorTree|SetBlackboardValueasVector (Variables|Default|GetKey) (Transformation|GetActorLocation (Utilities|Array|Get(acopy) (Variables|Default|GetP%20P) (Variables|Default|GetLCPI))))
    (Class|BTFunctionLibrary|SetBlackboardValueasInt _blackboardkeyselector (+ (Variables|Default|GetLCPI) 1)))
  (AI|BehaviorTree|FinishExecute true))