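; BP_Enemy is a battle-system enemy character that auto-attacks on a timer and plays combat montages.
; BeginPlay adds a SkeletMelee component, initializes it with RowName, stores it as CurrentHero and starts the looping CheckPlayer timer.
; CheckPlayer calls AutoAttack without detecting the player and picks a montage by RowName.
; Only row "3" has random hit reactions and a death montage that destroys the actor; player-trace and follow logic is disconnected.
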(event Custom|Hit
  ;[1 0.009744 0] ПОХУЙ ПОСТАВЬ  сюда поулчение урона я дальше разберусь,главнео что б анимации были, ну или нам будет больно ))
  (if (== (Variables|Default|GetRow%20Name) "3")
    (Animation|Montage|PlayMontage (Variables|Character|GetMesh) (Utilities|Select :Index (Math|Random|RandomInteger 2) :Option%200 (Variables|Default|GetAnim%20Montage1) :Option%201 (Variables|Default|GetAnim%20Montage2)))))

(event Custom|CheckPlayer
  ;[1 0 0.01454] Фигачь сюда монтаж,я после допишу логику, сюда автоатаку
  (Default|AutoAttack (stale EventBeginPlay _output_get) 1.0)
  (if (== (Variables|Default|GetRow%20Name) "3")
    ;[1 1 1] хз сработает ли
    (Animation|Montage|PlayMontage (Variables|Character|GetMesh) (Variables|Default|GetAnim%20MontageAttak) 1.7)
    (else
      (Animation|Montage|PlayMontage (Variables|Character|GetMesh) (Variables|Default|GetAnimMontageAOE)))))

(event Custom|DEATH
  (if (== (Variables|Default|GetRow%20Name) "3")
    (Animation|Montage|PlayMontage (Variables|Character|GetMesh) "/Game/Assets/CityofBrass_Enemies/Meshes/Enemy/Corpse/animation/eNEMYDEAD.eNEMYDEAD"
      (:OnCompleted
        (Actor|DestroyActor)))))

(event EventBeginPlay
  (bind _returnvalue (Game|AddComponentbyClass "/Game/AssetCore/Blueprints/BattleSystem/CharactersComponents/SkeletMelee.SkeletMelee_C"))
  (Variables|/Game/AssetCore/Blueprints/BattleSystem/CharactersComponents/ParentHeroComponent.ParentHeroComponent_C|SetRow%20Name _returnvalue (Variables|Default|GetRow%20Name))
  (Default|Initialization _returnvalue)
  (bind _output_get (Variables|Default|SetCurrent%20Hero _returnvalue))
  (Utilities|Time|SetTimerbyEvent (delegate Custom|CheckPlayer) 3.0 true -0.5))

(event EventTick
  (params (DeltaSeconds :type Float%20%28single-precision%29)))

(event Input|AxisEvents|InputAxisMoveForward/Backward
  (params (AxisValue :type Float%20%28single-precision%29))
  (Pawn|Input|AddMovementInput (Variables|Default|GetWorld%20Direction) AxisValue false))

(fn ConstructionScript)