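; BP_Player is the player character, swapping between heroes Amelia and Yars and handling movement, interaction and battle montages.
; InitChars fills the Chars map on BeginPlay and respawn; ChangeHero applies the chosen mesh, anim class and sword.
; Jumping polls a capsule trace for PhysicsBody ledges, then disables movement to hang.
; While hanging, WASD box-traces to adjacent holds, storing hand sockets; without a hold, up vaults and down drops.
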(event Custom|Hit%20Animation
  (bind _animmontageamelia (Variables|Default|GetAnimMontageAmelia))
  (Utilities|FlowControl|Sequence
    (:then_0
      (Animation|Montage|PlayMontage (Variables|Character|GetMesh) (Utilities|Select :Index (Math|Random|RandomInteger 2) :Option%200 _animmontageamelia :Option%201 _animmontageamelia)))
    (:then_1
      (Animation|Montage|PlayMontage (Variables|Character|GetMesh) (Utilities|Select :Index (Math|Random|RandomInteger 2) :Option%200 (Variables|Default|GetAnimMontage1) :Option%201 (Variables|Default|GetAnimMontage2))))))

(event Custom|Respawn
  (CallFunction|InitChars))

(event Custom|Jumpp
  (bind _self self)
  (bind _variable (|TemporaryVariable))
  (bind _capsulecomponent (Variables|Collision|GetCapsuleComponent))
  (bind _returnvalue (Transformation|GetActorLocation _self))
  (if (not (Variables|Default|GetHoop))
    (Character|Jump)
    (Default|CallJumpAnim)
    (|SetBy-RefVar _variable true)
    (if _variable :!label _label
      (Utilities|FlowControl|Sequence
        (:then_0
          (bind (_outhit _returnvalue_2) (Class|KismetSystemLibrary|CapsuleTraceSingleforObjects _returnvalue (+ _returnvalue (* (Transformation|GetActorForwardVector _self) 50)) 34.0 88.0 (Utilities|Array|MakeArray "ObjectTypeQuery4") false 0 "None" true "(R=1.000000,G=0.000000,B=0.000000,A=1.000000)" "(R=0.000000,G=1.000000,B=0.000000,A=1.000000)" 1.0))
          (if _returnvalue_2
            (Variables|Default|SetHoop true)
            (|SetBy-RefVar _variable false)))
        (:then_1
          (Utilities|FlowControl|Delay 0.1)
          (goto _label)))
      (elif (Variables|Default|GetHoop)
        (Utilities|Array|Add (Utilities|Array|MakeArray 0) (.HitActor (Collision|BreakHitResult _outhit)))
        (Components|MoveComponentTo _capsulecomponent (Math|Vector|MakeVector (.X (Math|Vector|BreakVector (.Location (Collision|BreakHitResult _outhit)))) (.Y (Math|Vector|BreakVector (.Location (Collision|BreakHitResult _outhit)))) (- (.z (Transformation|GetWorldLocation (.HitComponent (Collision|BreakHitResult _outhit)))) 8e+01)) (Math|Rotator|MakeRotator 0.0 0.0 (+ (.yaw (Math|Conversions|RotationFromXVector (.Normal (Collision|BreakHitResult _outhit)))) 1.8e+02)) false false 0.2 false)
        (Variables|Default|SetArray%20to%20ignore (Utilities|Array|MakeArray (.HitActor (Collision|BreakHitResult _outhit))))
        (Transformation|AddLocalOffset _capsulecomponent "10.000000, 0,-25.000000" false false)
        (Pawn|Components|CharacterMovement|SetMovementMode (Variables|Character|GetCharacterMovement) "MOVE_None" 0)
        (Variables|Default|SetRight%20 (Transformation|GetSocketLocation (.HitComponent (Collision|BreakHitResult _outhit)) "SocketR"))
        (Variables|Default|SetLeft%20 (Transformation|GetSocketLocation (.HitComponent (Collision|BreakHitResult _outhit)) "SocketL"))))))

(event Custom|YarsSkillOnGround
  (Animation|Montage|PlayMontage (Variables|Character|GetMesh) (Variables|Default|GetSkillOnGround) 2.0))

(event Custom|Change%20death
  (Utilities|FlowControl|Sequence
    (:then_0
      (Animation|Montage|PlayMontage (Variables|Character|GetMesh) "/Game/AssetCore/Models/Characters/Yars/Ani/Standing_Death_Backward_01__1__Montage.Standing_Death_Backward_01__1__Montage"
        (:OnCompleted
          (Utilities|FlowControl|Delay 0.02)
          (bind _keys (Utilities|Map|Keys (Variables|Default|GetChars)))
          (for _array_element _keys
            (CallFunction|ChangeHero _array_element)))))
    (:then_1
      (Animation|Montage|PlayMontage (Variables|Character|GetMesh) "/Game/AssetCore/Models/Characters/AmeliaFix/Animation/Dead_2.Dead_2"
        (:OnCompleted
          (Utilities|FlowControl|Delay 0.02)
          (bind _keys_2 (Utilities|Map|Keys (Variables|Default|GetChars)))
          (for _array_element_2 _keys_2
            (CallFunction|ChangeHero _array_element_2)))))))

(event Custom|AmeliaSkillOnAir
  (Animation|Montage|PlayMontage (Variables|Character|GetMesh) 0))

(event Custom|AmeliaSkillOnGround
  (Animation|Montage|PlayMontage (Variables|Character|GetMesh) (Variables|Default|GetUltimate)))

(event Custom|AmeliaUltimate
  (Animation|Montage|PlayMontage (Variables|Character|GetMesh) (Variables|Default|GetSkillOn%20Ground)))

(event EventBeginPlay
  (CallFunction|InitChars)
  (EventDispatchers|BindEventtoReapswn (delegate Custom|Respawn))
  (bind _asbp_player_controller (Utilities|Casting|CastToBP_PlayerController (Game|GetPlayerController 0)))
  (EventDispatchers|BindEventtoJump _asbp_player_controller (delegate Custom|Jumpp)))

(event Input|ActionEvents|InputActionSprint
  (params (Key :type Key%20Structure))
  (bind _charactermovement (Variables|Character|GetCharacterMovement))
  (:Pressed
    (Variables|/Script/Engine.CharacterMovementComponent|SetMaxWalkSpeed _charactermovement 8e+02))
  (:Released
    (Variables|/Script/Engine.CharacterMovementComponent|SetMaxWalkSpeed _charactermovement 4e+02)))

(event Input|ActionEvents|InputActionCrouch
  (params (Key :type Key%20Structure))
  (:Pressed
    (Character|Crouch)
    (Default|CallCrouchAnim)
    (Variables|Default|SetIsCrouch true))
  (:Released
    (Character|UnCrouch)
    (Default|CallUnCrouchAnim)
    (Variables|Default|SetIsCrouch false)))

(event Input|ActionEvents|InputActionLoockDown
  (params (Key :type Key%20Structure))
  ;[1 0.4574 0.4873] ОТКЛЮЧЕНО. Опускание головы
)

(event Input|ActionEvents|InputActionInteract
  (params (Key :type Key%20Structure))
  ;[1 1 1] Интерактивность(Внимание костыль)
  (:Pressed
    (for _array_element (Collision|GetOverlappingActors (Variables|Collision|GetCapsuleComponent) 0 :!class /Script/Engine.PrimitiveComponent)
      (Class|Interaction|Interaction(Message) _array_element))))

(event Input|AxisEvents|InputAxisMoveForward/Backward
  (params (AxisValue :type Float%20%28single-precision%29))
  (Pawn|Input|AddMovementInput (Variables|Default|GetWorld%20Direction) AxisValue false))

(event Input|KeyboardEvents|W
  (params (Key :type Key%20Structure))
  (:Pressed
    (if (Variables|Default|GetHoop)
      (Utilities|HoopTrace (Variables|Default|GetTrace) "NewEnumerator0"))))

(event Input|KeyboardEvents|A
  (params (Key :type Key%20Structure))
  (:Pressed
    (if (Variables|Default|GetHoop)
      (Utilities|HoopTrace (Variables|Default|GetTrace) "NewEnumerator3"))))

(event Input|KeyboardEvents|S
  (params (Key :type Key%20Structure))
  (:Pressed
    (if (Variables|Default|GetHoop)
      (Utilities|HoopTrace (Variables|Default|GetTrace) "NewEnumerator1"))))

(event Input|KeyboardEvents|D
  (params (Key :type Key%20Structure))
  (:Pressed
    (if (Variables|Default|GetHoop)
      (Utilities|HoopTrace (Variables|Default|GetTrace) "NewEnumerator2"))))

(fn ConstructionScript
  (Variables|/Script/Engine.SpringArmComponent|SetbDoCollisionTest (Variables|Default|GetSpringArm) false))

(fn ChangeHero
  (params (HeroSlot :type Integer))
  (bind _chars (Variables|Default|GetChars))
  (bind _sword_amelia (Variables|Default|GetSword%20Amelia))
  (bind _sword_yars (Variables|Default|GetSword%20Yars))
  (bind _value (Utilities|Map|Find _chars HeroSlot))
  (if (Utilities|IsValid _value)
    (Variables|Default|SetCurrent%20Hero HeroSlot)
    (Components|SkinnedMesh|SetSkinnedAssetandUpdate (Variables|Character|GetMesh) (Variables|/Game/AssetCore/Blueprints/BattleSystem/CharactersComponents/ParentHeroComponent.ParentHeroComponent_C|GetSet%20Model _value) true)
    (Class|SkeletalMeshComponent|SetAnimClass (Variables|Character|GetMesh) (Variables|/Game/AssetCore/Blueprints/BattleSystem/CharactersComponents/ParentHeroComponent.ParentHeroComponent_C|GetOut%20Row%20Anim%20Class _value))
    (Default|CallChangeHeroDispatch)
    (Math|Integer|CompareInt (Variables|Default|GetCurrent%20Hero)
      (:>
        (Rendering|SetVisibility _sword_amelia false false)
        (Rendering|SetVisibility _sword_yars true false))
      (:==
        (Rendering|SetVisibility _sword_yars false false)
        (Rendering|SetVisibility _sword_amelia true false)))))

(fn InitChars
  (bind _chars (Variables|Default|GetChars))
  (Utilities|FlowControl|Sequence
    (:then_0
      (bind _returnvalue (Game|AddComponentbyClass "/Game/AssetCore/Blueprints/BattleSystem/CharactersComponents/Amelia.Amelia_C"))
      (Default|Initialization _returnvalue)
      (Utilities|Map|Add _chars 0 _returnvalue))
    (:then_1
      (bind _returnvalue_2 (Game|AddComponentbyClass "/Game/AssetCore/Blueprints/BattleSystem/CharactersComponents/Yars.Yars_C"))
      (Variables|/Game/AssetCore/Blueprints/BattleSystem/CharactersComponents/ParentHeroComponent.ParentHeroComponent_C|SetRow%20Name _returnvalue_2 "2")
      (Default|Initialization _returnvalue_2)
      (Utilities|Map|Add _chars 1 _returnvalue_2))
    (:then_2
      (CallFunction|ChangeHero))))

(fn GetCurrentHero
  (return (.Value (Utilities|Map|Find (Variables|Default|GetChars) (Variables|Default|GetCurrent%20Hero)))))