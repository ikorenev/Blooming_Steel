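; BP_IzometriaCamera is the player-controlled isometric camera that also manages a two-hero party.
; On BeginPlay it spawns two BP_IzometriaPlayer actors at PlayerStart, adds Amelia and Edmund hero components, then activates and follows Amelia.
; Movement, relative to the camera's Arrow, and attack inputs go to the active player, while zoom and click-drag rotation drive the camera.
; ChangeCameraFollow switches the active hero and retargets the follow.
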(event EventBeginPlay
  (CallFunction|InitCamera))

(event Collision|EventActorBeginOverlap
  (params (OtherActor :type Actor%20Object%20Reference)))

(event EventTick
  (params (DeltaSeconds :type Float%20%28single-precision%29)))

(event Input|ActionEvents|InputActionMouseClick
  (params (Key :type Key%20Structure :default "None"))
  (:Pressed
    (Variables|Default|SetCanRotate true))
  (:Released
    (Variables|Default|SetCanRotate false)))

(event Input|ActionEvents|InputActionSpecialMove
  (params (Key :type Key%20Structure :default "None"))
  (:Pressed
    (if (not (Variables|Default|GetDelayForSpecialMove))
      (Variables|Default|SetDelayForSpecialMove true)
      (Default|SpecialMove (Variables|/Game/AssetCore/Blueprints/Core/BP_IzometriaPlayer.BP_IzometriaPlayer_C|GetHeroComponent (Variables|Default|GetActivePlayer)))
      (Utilities|FlowControl|Delay 0.5)
      (Variables|Default|SetDelayForSpecialMove false))))

(event Input|ActionEvents|InputActionAttackCharge
  (params (Key :type Key%20Structure :default "None"))
  (:Pressed
    (Default|ChargeAttack (Variables|/Game/AssetCore/Blueprints/Core/BP_IzometriaPlayer.BP_IzometriaPlayer_C|GetHeroComponent (Variables|Default|GetActivePlayer)))))

(event Input|ActionEvents|InputActionNormalAttack
  (params (Key :type Key%20Structure :default "None"))
  (:Pressed
    (Default|NormalAttack (Variables|/Game/AssetCore/Blueprints/Core/BP_IzometriaPlayer.BP_IzometriaPlayer_C|GetHeroComponent (Variables|Default|GetActivePlayer)))))

(event Input|AxisEvents|InputAxisMoveRight/Left
  (params (AxisValue :type Float%20%28single-precision%29))
  (Default|MoveSide (Variables|Default|GetActivePlayer) AxisValue (Math|Vector|GetRightVector (Variables|Default|GetArrow))))

(event Input|AxisEvents|InputAxisZoom
  (params (AxisValue :type Float%20%28single-precision%29))
  (Class|UniversalCamera|Zoomin AxisValue 1.0))

(event Input|AxisEvents|InputAxisMoveForward/Backward
  (params (AxisValue :type Float%20%28single-precision%29))
  (Default|MoveFront (Variables|Default|GetActivePlayer) AxisValue (Math|Vector|GetForwardVector (Variables|Default|GetArrow))))

(event Input|AxisEvents|InputAxisMouseAxisY
  (params (AxisValue :type Float%20%28single-precision%29))
  (if (Variables|Default|GetCanRotate)
    (Class|UniversalCamera|RotatePitch AxisValue -1.2 false)))

(event Input|AxisEvents|InputAxisMouseAxisX
  (params (AxisValue :type Float%20%28single-precision%29))
  (if (Variables|Default|GetCanRotate)
    (Class|UniversalCamera|RotateYaw AxisValue -1.2 false)))

(fn ConstructionScript)

(fn ChangeCameraFollow
  (params (Player :type Integer))
  (CallFunction|ChangePlayer Player)
  (CallFunction|FollowActivePlayer))

(fn InitCamera
  (bind _returnvalue (Actor|GetActorOfClass "/Script/Engine.PlayerStart"))
  (Utilities|FlowControl|Sequence
    (:then_0
      (bind _returnvalue_2 (Game|SpawnActorfromClass "/Game/AssetCore/Blueprints/Core/BP_IzometriaPlayer.BP_IzometriaPlayer_C" (Math|Transform|MakeTransform (Transformation|GetActorLocation _returnvalue) "0, 0, 0" "1.000000,1.000000,1.000000") "Undefined" 0 0))
      (bind _returnvalue_3 (Game|AddComponentbyClass _returnvalue_2 "/Game/AssetCore/Blueprints/BattleSystem/CharactersComponents/Amelia.Amelia_C"))
      (Variables|/Game/AssetCore/Blueprints/Core/BP_IzometriaPlayer.BP_IzometriaPlayer_C|SetHeroComponent _returnvalue_2 _returnvalue_3)
      (bind _output_get (Variables|Default|SetСurrentPlayer1 _returnvalue_2))
      (bind _output_get_2 (Variables|Default|SetActivePlayer _output_get))
      (Default|ActiveHero _output_get_2)
      (CallFunction|FollowActivePlayer))
    (:then_1
      (bind _returnvalue_4 (Game|SpawnActorfromClass "/Game/AssetCore/Blueprints/Core/BP_IzometriaPlayer.BP_IzometriaPlayer_C" (Math|Transform|MakeTransform (- (Transformation|GetActorLocation _returnvalue) "100.000000,100.000000,0.000000") "0, 0, 0" "1.000000,1.000000,1.000000") "Undefined" 0 0))
      (bind _output_get_3 (Variables|Default|SetСurrentPlayer2 _returnvalue_4))
      (bind _returnvalue_5 (Game|AddComponentbyClass _output_get_3 "/Game/AssetCore/Blueprints/BattleSystem/CharactersComponents/Edmund.Edmund_C"))
      (Variables|/Game/AssetCore/Blueprints/Core/BP_IzometriaPlayer.BP_IzometriaPlayer_C|SetHeroComponent _output_get_3 _returnvalue_5))))

(fn ChangePlayer
  (params (Player :type Integer))
  (switch int Player
    (:1
      (Default|DeactiveHero (Variables|Default|GetActivePlayer))
      (bind _output_get (Variables|Default|SetActivePlayer (Variables|Default|GetСurrentPlayer1)))
      (Default|ActiveHero _output_get))
    (:2
      (Default|DeactiveHero (Variables|Default|GetActivePlayer))
      (bind _output_get_2 (Variables|Default|SetActivePlayer (Variables|Default|GetСurrentPlayer2)))
      (Default|ActiveHero _output_get_2))))

(fn FollowActivePlayer
  (Class|UniversalCamera|FollowTarget :TargetSettings (Class|UniversalCamera|UseActor (Variables|Default|GetActivePlayer))))