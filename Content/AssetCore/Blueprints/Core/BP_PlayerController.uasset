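; Player controller that routes input for a hero-switching party system to BP_Player and its current hero.
; Four hero keys pass a slot index to ChangeHero, while attack, skill and ultimate inputs act on the current hero, with the two attacks also calling animations on BP_Player.
; FlipFlops toggle the party-selection streamed level and the M-key teleport widget.
; Jump fires only when the character is not falling.
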(event EventBeginPlay)

(event EventTick
  (params (DeltaSeconds :type Float%20%28single-precision%29)))

(event Input|ActionEvents|InputActionHero1
  (params (Key :type Key%20Structure))
  (:Pressed
    (Variables|Default|SetHero%20Slot 0)
    (bind _asbp_player (Utilities|Casting|CastToBP_Player (Game|GetPlayerCharacter 0)))
    (Default|ChangeHero _asbp_player (Variables|Default|GetHero%20Slot))))

(event Input|ActionEvents|InputActionHero2
  (params (Key :type Key%20Structure))
  (:Pressed
    (Variables|Default|SetHero%20Slot 1)
    (bind _asbp_player (Utilities|Casting|CastToBP_Player (Game|GetPlayerCharacter 0)))
    (Default|ChangeHero _asbp_player (Variables|Default|GetHero%20Slot))))

(event Input|ActionEvents|InputActionUltimate
  (params (Key :type Key%20Structure))
  (:Pressed
    (bind _asbp_player (Utilities|Casting|CastToBP_Player (Game|Player|GetPlayerPawn 0)))
    (bind _newparam (Default|GetCurrentHero _asbp_player))
    (Default|Ultimate _newparam)))

(event Input|ActionEvents|InputActionHero3
  (params (Key :type Key%20Structure))
  (:Pressed
    (Variables|Default|SetHero%20Slot 2)
    (bind _asbp_player (Utilities|Casting|CastToBP_Player (Game|GetPlayerCharacter 0)))
    (Default|ChangeHero _asbp_player (Variables|Default|GetHero%20Slot))))

(event Input|ActionEvents|InputActionHero4
  (params (Key :type Key%20Structure))
  (:Pressed
    (Variables|Default|SetHero%20Slot 3)
    (bind _asbp_player (Utilities|Casting|CastToBP_Player (Game|GetPlayerCharacter 0)))
    (Default|ChangeHero _asbp_player (Variables|Default|GetHero%20Slot))))

(event Input|ActionEvents|InputActionSelectParty
  (params (Key :type Key%20Structure))
  (:Pressed
    (Utilities|FlowControl|FlipFlop
      (:A
        (Class|GameplayStatics|LoadStreamLevelbySoftObjectPtr "/Game/Maps/ChangeHero.ChangeHero" true false)
        (Default|CallSetParty))
      (:B
        (Class|GameplayStatics|UnloadStreamLevelbySoftObjectPtr "/Game/Maps/ChangeHero.ChangeHero" false)
        (Default|CallReturnGame)))))

(event Input|ActionEvents|InputActionAttack
  (params (Key :type Key%20Structure))
  (:Pressed
    (bind _asbp_player (Utilities|Casting|CastToBP_Player (Game|Player|GetPlayerPawn 0)))
    (bind _newparam (Default|GetCurrentHero _asbp_player))
    (Default|AutoAttack _newparam 1.0)
    (Default|CallAttackAnim _asbp_player)))

(event Input|ActionEvents|InputActionJump
  (params (Key :type Key%20Structure))
  (bind _returnvalue (Game|GetPlayerCharacter 0))
  (:Pressed
    (if (Utilities|Enum|NotEqual(Enum) (Variables|/Script/Engine.CharacterMovementComponent|GetMovementMode (Variables|/Script/Engine.Character|GetCharacterMovement _returnvalue)) "MOVE_Falling")
      (Default|CallJump)))
  (:Released
    (Character|StopJumping _returnvalue)))

(event Input|ActionEvents|InputActionSkillAttack(1)
  (params (Key :type Key%20Structure))
  (:Pressed
    (bind _asbp_player (Utilities|Casting|CastToBP_Player (Game|Player|GetPlayerPawn 0)))
    (bind _newparam (Default|GetCurrentHero _asbp_player))
    (Default|SkillAttack _newparam)
    (Default|CallSkillAttackAnim _asbp_player)))

(event Input|ActionEvents|InputActionSkillMove(2)
  (params (Key :type Key%20Structure))
  (:Pressed
    (bind _asbp_player (Utilities|Casting|CastToBP_Player (Game|Player|GetPlayerPawn 0)))
    (bind _newparam (Default|GetCurrentHero _asbp_player))
    (Default|SkillMove _newparam)))

(event Input|KeyboardEvents|M
  (params (Key :type Key%20Structure))
  (:Pressed
    (Utilities|FlowControl|FlipFlop
      (:A
        (bind _returnvalue (UserInterface|CreateWidget "/Game/AssetCore/UI/ControlTeleport.ControlTeleport_C"))
        (UserInterface|Viewport|AddtoViewport _returnvalue 0))
      (:B
        (Widget|RemovefromParent _returnvalue)))))

(fn ConstructionScript)