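; Main game HUD that creates the main UI and an interaction prompt widget at BeginPlay, adding only the main UI to the viewport.
; InteractOnDisplay shows the prompt at the player pawn's projected screen position plus a fixed offset, set once per call, and HideInteract removes it.
; HideALL and ShowAll toggle MainBattleUI visibility, but that widget's creation is disconnected and never runs here.
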(event EventBeginPlay
  (bind _returnvalue (UserInterface|CreateWidget "/Game/AssetCore/UI/BattleUI/MainUI.MainUI_C"))
  (Variables|Default|SetMainUI _returnvalue)
  (UserInterface|Viewport|AddtoViewport _returnvalue 0)
  (bind _returnvalue_2 (UserInterface|CreateWidget "/Game/AssetCore/UI/Interaction.Interaction_C"))
  (Variables|Default|SetInteraction _returnvalue_2))

(event Collision|EventActorBeginOverlap
  (params (OtherActor :type Actor%20Object%20Reference)))

(event EventTick
  (params (DeltaSeconds :type Float%20%28single-precision%29)))

(fn ConstructionScript)

(fn HideALL
  (Widget|SetVisibility (Variables|Default|GetMainBattleUI) "Hidden"))

(fn ShowAll
  (Widget|SetVisibility (Variables|Default|GetMainBattleUI) "Visible"))

(fn HideInteract
  (Widget|RemovefromParent (Variables|Default|GetInteraction)))

(fn InteractonDisplay
  (bind _interaction (Variables|Default|GetInteraction))
  (UserInterface|Viewport|AddtoViewport _interaction 0)
  (Class|UserWidget|SetPositioninViewport _interaction (+ (.ScreenPosition (Class|GameplayStatics|ProjectWorldtoScreen (Game|GetPlayerController 0) (Transformation|GetActorLocation (Game|Player|GetPlayerPawn 0)) false)) "(X=-20.000000,Y=-350.000000)") true))