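; Isometric player character with world-axis movement, sprint, crouch, hit and death montages, and interaction messages sent to overlapping actors.
; While Hoop is set, WASD calls HoopTrace, which box-traces for neighboring ledges to move onto, or climbs up or drops off when none is found.
; The jump and capsule-trace ledge grab that sets Hoop is disconnected, as are head-lowering timelines.
; InitChars and the timed Interact event are empty stubs.
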(event Custom|Hit%20Animation
  (Animation|Montage|PlayMontage (Variables|Character|GetMesh) (Utilities|Select :Index (Math|Random|RandomInteger 2) :Option%200 (Variables|Default|GetAnimMontage1) :Option%201 (Variables|Default|GetAnimMontage2))))

(event Custom|Respawn
  (CallFunction|InitChars))

(event Custom|Jumpp)

(event Custom|Change%20death
  (Animation|Montage|PlayMontage (Variables|Character|GetMesh) "/Game/AssetCore/Blueprints/Animation/Standing_Death_Backward_01__1__Montage.Standing_Death_Backward_01__1__Montage"
    (:OnCompleted
      (Utilities|FlowControl|Delay 0.02))))

(event Custom|MoveSide
  (params (Axis :type Float%20%28double-precision%29))
  (Pawn|Input|AddMovementInput "0.000000,1.000000,0.000000" Axis false))

(event Custom|Move%20Front
  (params (Axis :type Float%20%28double-precision%29))
  (Pawn|Input|AddMovementInput "1.000000,0.000000,0.000000" Axis false))

(event Custom|ActiveHero
  (Utilities|Time|SetTimerbyEvent (delegate Custom|Interact) 0.05 true))

(event Custom|Interact)

(event EventBeginPlay
  (Utilities|Time|SetTimerbyFunctionName 0 "CameraHide" 0.2 true -0.2)
  (CallFunction|InitChars)
  (EventDispatchers|BindEventtoReapswn (delegate Custom|Respawn)))

(event Input|ActionEvents|InputActionSprint
  (params (Key :type Key%20Structure :default "None"))
  (bind _charactermovement (Variables|Character|GetCharacterMovement))
  (:Pressed
    (Variables|/Script/Engine.CharacterMovementComponent|SetMaxWalkSpeed _charactermovement 8e+02))
  (:Released
    (Variables|/Script/Engine.CharacterMovementComponent|SetMaxWalkSpeed _charactermovement 4e+02)))

(event Input|ActionEvents|InputActionCrouch
  (params (Key :type Key%20Structure :default "None"))
  (:Pressed
    (Character|Crouch)
    (Default|CallCrouchAnim)
    (Variables|Default|SetIsCrouch true))
  (:Released
    (Character|UnCrouch)
    (Default|CallUnCrouchAnim)
    (Variables|Default|SetIsCrouch false)))

(event Input|ActionEvents|InputActionLoockDown
  (params (Key :type Key%20Structure :default "None"))
  ;[1 0.4574 0.4873] ОТКЛЮЧЕНО. Опускание головы
)

(event Input|ActionEvents|InputActionInteract
  (params (Key :type Key%20Structure :default "None"))
  ;[1 1 1] Интерактивность(Внимание костыль)
  (:Pressed
    (for _array_element (Collision|GetOverlappingActors (Variables|Collision|GetCapsuleComponent) 0 :!class /Script/Engine.PrimitiveComponent)
      (Class|Interact|Interaction(Message) _array_element))))

(event Input|KeyboardEvents|W
  (params (Key :type Key%20Structure :default "None"))
  (:Pressed
    (if (Variables|Default|GetHoop)
      (Utilities|HoopTrace (Variables|Default|GetTrace) "NewEnumerator0"))))

(event Input|KeyboardEvents|A
  (params (Key :type Key%20Structure :default "None"))
  (:Pressed
    (if (Variables|Default|GetHoop)
      (Utilities|HoopTrace (Variables|Default|GetTrace) "NewEnumerator3"))))

(event Input|KeyboardEvents|S
  (params (Key :type Key%20Structure :default "None"))
  (:Pressed
    (if (Variables|Default|GetHoop)
      (Utilities|HoopTrace (Variables|Default|GetTrace) "NewEnumerator1"))))

(event Input|KeyboardEvents|D
  (params (Key :type Key%20Structure :default "None"))
  (:Pressed
    (if (Variables|Default|GetHoop)
      (Utilities|HoopTrace (Variables|Default|GetTrace) "NewEnumerator2"))))

(fn ConstructionScript
  (Variables|/Script/Engine.SpringArmComponent|SetbDoCollisionTest (Variables|Default|GetSpringArm) false))

(fn InitChars)