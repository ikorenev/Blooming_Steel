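; Amelia is a character-specific ability Blueprint that acts on its owning Character, overriding skill functions from a parent class.
; Ultimate and AutoAttack only call the parent, and PKM is empty.
; SkillOnAir adds an upward impulse to the parent behavior, then lowers gravity scale and air control for a floaty state.
; A looping timer polls OnAirCheck to raise gravity once not falling; air control stays unrestored and the timer is never cleared.
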(event EventBeginPlay
  (|CallParentFunction) ; This node is disabled and will not be called.\nDrag off pins to build functionality.
)

(event EventTick
  (params (DeltaSeconds :type Float%20%28single-precision%29))
  (|CallParentFunction DeltaSeconds) ; This node is disabled and will not be called.\nDrag off pins to build functionality.
)

(fn Ultimate
  (|CallParentFunction))

(fn AutoAttack
  (params (Multiply :type Float%20%28double-precision%29))
  (|CallParentFunction Multiply))

(fn PKM)

(fn SkillonAir
  (|CallParentFunction)
  (bind _ascharacter (Utilities|Casting|CastToCharacter (Components|GetOwner)))
  (Physics|AddImpulse (Variables|/Script/Engine.Character|GetCharacterMovement _ascharacter) (Math|Vector|MakeVector 0.0 0.0 3e+02) true)
  (Variables|/Script/Engine.CharacterMovementComponent|SetGravityScale (Variables|/Script/Engine.Character|GetCharacterMovement _ascharacter) 0.5)
  (Variables|/Script/Engine.CharacterMovementComponent|SetAirControl (Variables|/Script/Engine.Character|GetCharacterMovement _ascharacter) 0.05)
  (Utilities|Time|SetTimerbyFunctionName 0 "OnAirCheck" 0.1 true))

(fn OnAirCheck
  (bind _ascharacter (Utilities|Casting|CastToCharacter (Components|GetOwner)))
  (if (not (AI|Components|NavMovement|IsFalling (Variables|/Script/Engine.Character|GetCharacterMovement _ascharacter)))
    (Variables|/Script/Engine.CharacterMovementComponent|SetGravityScale (Variables|/Script/Engine.Character|GetCharacterMovement _ascharacter) 2.0)))