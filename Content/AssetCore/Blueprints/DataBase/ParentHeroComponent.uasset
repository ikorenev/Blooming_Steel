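; Base hero component for player and enemy characters, handling stats, combat and death.
; Initialization loads stats, skills and mesh from a data table row by name.
; Skills fire dispatchers when ready, with Ultimate also spending energy, while auto attack box-traces the opposing side.
; Damage subtracts typed defense (except true damage), shows damage numbers, then destroys dead enemies or switches the player's hero, showing a death screen when none remain.
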(event EventBeginPlay)

(fn Initialization
  (bind _returnvalue (Utilities|GetDataTableRow "/Game/AssetCore/Blueprints/DataBase/Heroes.Heroes" (Variables|Default|GetRow%20Name))
    (:then
      (Utilities|FlowControl|Sequence
        (:then_0
          (bind _output_get (Variables|Default|SetMaxHp (.maxhp _returnvalue)))
          (Variables|Default|SetCurrentHP _output_get))
        (:then_1
          (Variables|Default|SetPhisDef (.phisdef _returnvalue)))
        (:then_2
          (Variables|Default|SetMageDef (.magedef _returnvalue)))
        (:then_3
          (Variables|Default|SetPhisDamage (.phisdamage _returnvalue)))
        (:then_4
          (Variables|Default|SetMageDamage (.magedamage _returnvalue)))
        (:then_5
          (Variables|Default|SetSpeedChar (.speedchar _returnvalue)))
        (:then_6
          (Variables|Default|SetAttackSpeed (.attackspeed _returnvalue)))
        (:then_7
          (Variables|Default|SetCritRate (.critrate _returnvalue)))
        (:then_8
          (Variables|Default|SetCritDamage (.critdamage _returnvalue)))
        (:then_9
          (Variables|Default|SetEnergyRecharge (.energyrecharge _returnvalue)))
        (:then_10
          (Variables|Default|SetTimeSkillCD (.timeskillcd _returnvalue)))
        (:then_11
          (Variables|Default|SetHealPower (.healpower _returnvalue)))
        (:then_12
          (Variables|Default|SetUltimateCost (.ultimatecost _returnvalue))
          (Variables|Default|SetEnergy 0.0))
        (:then_13
          (bind _output_get_2 (Variables|Default|SetSet%20Model (.heromodels _returnvalue)))
          (bind _ascharacter (Utilities|Casting|CastToCharacter (Components|GetOwner)))
          (Class|SkinnedMeshComponent|SetSkeletalMesh (Variables|/Script/Engine.Character|GetMesh _ascharacter) _output_get_2 true)
          (Variables|Default|SetOut%20Row%20Anim%20Class (.animclass _returnvalue)))
        (:then_14
          (Variables|Default|SetNameChar (.name _returnvalue)))
        (:then_15
          (Variables|Default|SetCD_SkillAttack (.cd_skillattack _returnvalue))
          (Variables|Default|SetCD_SkillMove (.cd_skillmove _returnvalue))
          (Variables|Default|SetCD_Ultimate (.cd_ultimate _returnvalue)))
        (:then_16
          (Variables|Default|SetOut%20Row%20Skill%20Attack (.skillattack _returnvalue))
          (Variables|Default|SetOut%20Row%20Skill%20Move (.skillmove _returnvalue))
          (Variables|Default|SetOut%20Row%20Ultimate (.ultimate _returnvalue))
          (Variables|Default|SetHP_BarImage (.imageleft _returnvalue)))))))

(fn SkillAttack
  (if (Variables|Default|GetSkillAttackReady)
    (Default|CallSkillAttackUse)
    (return)))

(fn SkillMove
  (if (Variables|Default|GetSkillMoveReady)
    (Default|CallSkillMoveUse)))

(fn Ultimate
  (if (Variables|Default|GetUltimateReady)
    (if (>= (Variables|Default|GetEnergy) (Variables|Default|GetUltimateCost))
      (Variables|Default|SetEnergy (- (Variables|Default|GetEnergy) (Variables|Default|GetUltimateCost)))
      (Default|CallUltimateUse))))

(fn AutoAttack
  (params (Multiply :type Float%20%28double-precision%29))
  (bind _returnvalue (Components|GetOwner))
  (bind _returnvalue_2 (Components|GetOwner))
  (bind _phisdamage (Variables|Default|GetPhisDamage))
  (bind _returnvalue_3 (Transformation|GetActorLocation _returnvalue_2))
  (bind _returnvalue_4 (* _phisdamage Multiply))
  (bind _outhit (Class|KismetSystemLibrary|BoxTraceSingleforObjects _returnvalue_3 (+ _returnvalue_3 (* (Transformation|GetActorForwardVector _returnvalue_2) "1.000000,100.000000,1.000000")) "30.000000,30.000000,90.000000" "0, 0, 0" (Variables|Default|GetObject%20Types) false 0 "None" true))
  (Utilities|Casting|CastToBP_Player _returnvalue
    (:then
      (bind _asbp_enemy (Utilities|Casting|CastToBP_Enemy (.HitActor (Collision|BreakHitResult _outhit))))
      (CallFunction|TakeDamage (Variables|/Game/AssetCore/Blueprints/Core/BP_Enemy.BP_Enemy_C|GetCurrent%20Hero _asbp_enemy) _returnvalue_4 "NewEnumerator0" false))
    (:CastFailed
      (Utilities|Casting|CastToBP_Enemy _returnvalue)
      (bind _asbp_player (Utilities|Casting|CastToBP_Player (.HitActor (Collision|BreakHitResult _outhit))))
      (bind _newparam (Default|GetCurrentHero _asbp_player))
      (CallFunction|TakeDamage _newparam _returnvalue_4 "NewEnumerator0" false))))

(fn TakeDamage
  (params (Damage :type Float%20%28double-precision%29) (TypeDamage :type DamageType%20Enum :default "NewEnumerator0") (ScreenDamage :type Boolean))
  (bind _magedef (Variables|Default|GetMageDef))
  (bind _phisdef (Variables|Default|GetPhisDef))
  (bind _returnvalue (- Damage _magedef))
  (bind _returnvalue_2 (- Damage _phisdef))
  (bind _returnvalue_3 (Math|Float|Clamp(Float) _returnvalue_2 0.0 Damage))
  (bind _returnvalue_4 (Math|Float|Clamp(Float) _returnvalue 0.0 Damage))
  (LocalVariables|SetSetScreenDamage (not ScreenDamage))
  (switch Utilities|FlowControl|Switch|SwitchonDamageType TypeDamage
    (:NewEnumerator0
      (CallFunction|SetDamage (Math|Float|Clamp(Float) _returnvalue_3 0.0 (Variables|Default|GetCurrentHP)) (LocalVariables|GetSetScreenDamage))
      (Variables|Default|SetCurrentHP (Math|Float|Clamp(Float) (- (Variables|Default|GetCurrentHP) _returnvalue_3) 0.0 (Variables|Default|GetCurrentHP))))
    (:NewEnumerator1
      (CallFunction|SetDamage (Math|Float|Clamp(Float) _returnvalue_4 0.0 (Variables|Default|GetCurrentHP)) (LocalVariables|GetSetScreenDamage))
      (Variables|Default|SetCurrentHP (- (Variables|Default|GetCurrentHP) _returnvalue_4)))
    (:NewEnumerator2
      (CallFunction|SetDamage (Math|Float|Clamp(Float) Damage 0.0 (Variables|Default|GetCurrentHP)) (LocalVariables|GetSetScreenDamage))
      (Variables|Default|SetCurrentHP (- (Variables|Default|GetCurrentHP) Damage))))
  (bind _asbp_player (Utilities|Casting|CastToBP_Player (Components|GetOwner))
    (:then
      (Default|CallHitAnim _asbp_player)
      (Default|CallUpdateHPbar))
    (:CastFailed
      _))
  (CallFunction|Death?))

(fn Death?
  (bind _returnvalue (Components|GetOwner))
  (if (<= (Variables|Default|GetCurrentHP) 0.0)
    (Utilities|Casting|CastToBP_Enemy _returnvalue
      (:then
        (Actor|DestroyActor _returnvalue))
      (:CastFailed
        (bind _asbp_player (Utilities|Casting|CastToBP_Player _returnvalue))
        (Utilities|Map|Remove (Variables|/Game/AssetCore/Blueprints/Core/BP_Player.BP_Player_C|GetChars _asbp_player) (Variables|/Game/AssetCore/Blueprints/Core/BP_Player.BP_Player_C|GetCurrent%20Hero _asbp_player))
        (if (Utilities|Map|IsNotEmpty (Variables|/Game/AssetCore/Blueprints/Core/BP_Player.BP_Player_C|GetChars _asbp_player))
          (bind _keys (Utilities|Map|Keys (Variables|/Game/AssetCore/Blueprints/Core/BP_Player.BP_Player_C|GetChars _asbp_player)))
          (for _array_element _keys
            (Default|ChangeHero _asbp_player _array_element))
          (else
            (bind _returnvalue_2 (UserInterface|CreateWidget "/Game/UI/BattleUI/Death.Death_C"))
            (UserInterface|Viewport|AddtoViewport _returnvalue_2 0)))))))

(fn SetDamage
  (params (A :type Float%20%28double-precision%29) (ScreenDamage :type Boolean))
  (if ScreenDamage
    (bind _returnvalue (UserInterface|CreateWidget "/Game/UI/BattleUI/HitDamage.HitDamage_C"))
    (Class|UserWidget|SetPositioninViewport _returnvalue (+ (+ (.ScreenPosition (Class|GameplayStatics|ProjectWorldtoScreen (Game|GetPlayerController 0) (Transformation|GetActorLocation (Components|GetOwner)) false)) "(X=0.000000,Y=-120.000000)") (Math|Vector2D|MakeVector2D (Math|Random|RandomFloatinRange -3e+01 3e+01) (Math|Random|RandomFloatinRange -3e+01 3e+01))) true)
    (UserInterface|Viewport|AddtoViewport _returnvalue 0)
    (Default|GetDamage _returnvalue (Math|Float|Truncate A))))

(fn SetActiveWidget
  (params (TypeSkill :type TypeSkill%20Enum :default "NewEnumerator0") (index :type Integer))
  (bind _returnvalue (Actor|GetActorOfClass "/Game/AssetCore/Blueprints/Core/HUD_BattleUI.HUD_BattleUI_C"))
  (switch Utilities|FlowControl|Switch|SwitchonTypeSkill TypeSkill
    (:NewEnumerator0
      (Class|WidgetSwitcher|SetActiveWidgetIndex (Variables|/Game/UI/BattleUI/Skill.Skill_C|GetWidgetSwitcher_152 (Variables|/Game/UI/BattleUI/Skills.Skills_C|GetSkill_Attack (Variables|/Game/UI/BattleUI/MainBattleUI.MainBattleUI_C|GetSkills (Variables|/Game/AssetCore/Blueprints/Core/HUD_BattleUI.HUD_BattleUI_C|GetMainUI _returnvalue)))) index))
    (:NewEnumerator1
      (Class|WidgetSwitcher|SetActiveWidgetIndex (Variables|/Game/UI/BattleUI/Skill.Skill_C|GetWidgetSwitcher_152 (Variables|/Game/UI/BattleUI/Skills.Skills_C|GetSkill_Move (Variables|/Game/UI/BattleUI/MainBattleUI.MainBattleUI_C|GetSkills (Variables|/Game/AssetCore/Blueprints/Core/HUD_BattleUI.HUD_BattleUI_C|GetMainUI _returnvalue)))) index))
    (:NewEnumerator2
      (Class|WidgetSwitcher|SetActiveWidgetIndex (Variables|/Game/UI/BattleUI/Skill.Skill_C|GetWidgetSwitcher_152 (Variables|/Game/UI/BattleUI/Skills.Skills_C|GetUltimate (Variables|/Game/UI/BattleUI/MainBattleUI.MainBattleUI_C|GetSkills (Variables|/Game/AssetCore/Blueprints/Core/HUD_BattleUI.HUD_BattleUI_C|GetMainUI _returnvalue)))) index))))