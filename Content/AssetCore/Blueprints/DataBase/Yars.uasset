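; Yars is a child Blueprint, owned by BP_Player, that overrides the parent's air skill to perform a short forward dash.
; SkillOnAir runs the parent logic, then applies a velocity-change impulse along the player's forward vector through CharacterMovement.
; It then calls the Gravity event, which zeroes the player's velocity after a brief delay to cut the dash short, despite its name.
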(event Custom|Gravity
  (Utilities|FlowControl|Delay 0.15)
  (bind _asbp_player (Utilities|Casting|CastToBP_Player (Components|GetOwner)))
  (Variables|/Script/Engine.MovementComponent|SetVelocity (Variables|/Script/Engine.Character|GetCharacterMovement _asbp_player) "0, 0, 0"))

(event EventBeginPlay
  (|CallParentFunction) ; This node is disabled and will not be called.\nDrag off pins to build functionality.
)

(event EventTick
  (params (DeltaSeconds :type Float%20%28single-precision%29))
  (|CallParentFunction DeltaSeconds) ; This node is disabled and will not be called.\nDrag off pins to build functionality.
)

(fn SkillonAir
  (|CallParentFunction)
  (bind _asbp_player (Utilities|Casting|CastToBP_Player (Components|GetOwner)))
  (Physics|AddImpulse (Variables|/Script/Engine.Character|GetCharacterMovement _asbp_player) (* (Transformation|GetActorForwardVector _asbp_player) 4e+03) true)
  (CallFunction|Gravity))