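; Level-tool trigger volume that changes the player's camera distance when BP_Player enters its box.
; On overlap it plays a timeline that lerps the spring arm's current length toward NewTargetArmLength, compounding the blend each update.
; The construction script sets a timeline play rate from SpeedRate.
; Nothing restores the length on exit, and the timeline is played without being rewound.
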(event OnComponentBeginOverlap(Box)
  (params (OverlappedComponent :type Primitive%20Component%20Object%20Reference) (OtherActor :type Actor%20Object%20Reference) (OtherComp :type Primitive%20Component%20Object%20Reference) (OtherBodyIndex :type Integer) (bFromSweep :type Boolean) (SweepResult :type Hit%20Result%20Structure%20%28by%20ref%29))
  (bind _asbp_player (Utilities|Casting|CastToBP_Player OtherActor))
  (bind _newtrack_0 (Timeline|Timeline_0 Play)
    (:Update
      (Variables|/Script/Engine.SpringArmComponent|SetTargetArmLength (Variables|/Game/AssetCore/Blueprints/BattleSystem/CharactersClass/BP_Player.BP_Player_C|GetSpringArm _asbp_player) (Math|Float|Lerp (Variables|/Script/Engine.SpringArmComponent|GetTargetArmLength (Variables|/Game/AssetCore/Blueprints/BattleSystem/CharactersClass/BP_Player.BP_Player_C|GetSpringArm _asbp_player)) (Variables|Default|GetNewTarget%20Arm%20Length) _newtrack_0)))))

(event EventBeginPlay)

(event Collision|EventActorBeginOverlap
  (params (OtherActor :type Actor%20Object%20Reference)))

(event EventTick
  (params (DeltaSeconds :type Float%20%28single-precision%29)))

(fn ConstructionScript
  (Components|Timeline|SetPlayRate (Variables|Default|GetTimeline_0) (Variables|Default|GetSpeedRate)))