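; Camera trigger volume that changes the isometric camera's framing when the active BP_IzometriaPlayer enters its box.
; On overlap, a timeline blends the player-pawn camera's spring arm length and rotation toward the trigger's targets, re-reading current values each update.
; An IsMixed flag blocks retriggering until an overlap ends.
; The construction script applies the targets to its own spring arm and counter-transforms the child actor and box.
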(event OnComponentBeginOverlap(Box)
  (params (OverlappedComponent :type Primitive%20Component%20Object%20Reference) (OtherActor :type Actor%20Object%20Reference) (OtherComp :type Primitive%20Component%20Object%20Reference) (OtherBodyIndex :type Integer) (bFromSweep :type Boolean) (SweepResult :type Hit%20Result%20Structure%20%28by%20ref%29))
  (bind _asbp_izometria_player (Utilities|Casting|CastToBP_IzometriaPlayer OtherActor))
  (if (Variables|/Game/AssetCore/Blueprints/Core/BP_IzometriaPlayer.BP_IzometriaPlayer_C|GetisActive? _asbp_izometria_player)
    (if (not (Variables|Default|GetIsMixed))
      (Variables|Default|SetIsMixed true)
      (bind _asbp_izometria_camera (Utilities|Casting|CastToBP_IzometriaCamera (Game|Player|GetPlayerPawn 0)))
      (bind _newtrack_0 (Timeline|Timeline PlayFromStart)
        (:Update
          (CallFunction|MixCamera _asbp_izometria_camera _newtrack_0))))))

(event OnComponentEndOverlap(Box)
  (params (OverlappedComponent :type Primitive%20Component%20Object%20Reference) (OtherActor :type Actor%20Object%20Reference) (OtherComp :type Primitive%20Component%20Object%20Reference) (OtherBodyIndex :type Integer))
  (Variables|Default|SetIsMixed false))

(event EventBeginPlay)

(event Collision|EventActorBeginOverlap
  (params (OtherActor :type Actor%20Object%20Reference)))

(event EventTick
  (params (DeltaSeconds :type Float%20%28single-precision%29)))

(fn ConstructionScript
  (bind _childactor (Variables|Default|GetChildActor))
  (bind _new_rotation (Variables|Default|GetNew%20Rotation))
  (bind _target_arm_length (Variables|Default|GetTarget%20Arm%20Length))
  (bind _springarmcomponent (Variables|Default|GetSpringArmComponent))
  (bind _returnvalue (* _new_rotation -1.0))
  (Transformation|SetRelativeRotation _springarmcomponent _new_rotation false false)
  (Variables|/Script/Engine.SpringArmComponent|SetTargetArmLength _springarmcomponent _target_arm_length)
  (Transformation|SetRelativeRotation _childactor _returnvalue false false)
  (Transformation|SetRelativeLocation _childactor (Math|Vector|MakeVector _target_arm_length 0.0 0.0) false false)
  (Transformation|SetRelativeTransform (Variables|Default|GetBox) (Math|Transform|MakeTransform (Math|Vector|MakeVector _target_arm_length 0.0 0.0) _returnvalue (Variables|Default|GetNew%20Scale%203D)) false false))

(fn MixCamera
  (params (self2 :type Universal%20Camera%20Object%20Reference) (Alpha :type Float%20%28single-precision%29))
  (bind _springarmcomponent (Variables|/Script/UniversalCameraPlugin.UniversalCamera|GetSpringArmComponent self2))
  (Utilities|FlowControl|Sequence
    (:then_0
      (LocalVariables|SetTargetArmLenght (Variables|/Script/Engine.SpringArmComponent|GetTargetArmLength _springarmcomponent))
      (LocalVariables|SetRelativeRotation (Variables|/Script/Engine.SceneComponent|GetRelativeRotation _springarmcomponent)))
    (:then_1
      (Variables|/Script/Engine.SpringArmComponent|SetTargetArmLength _springarmcomponent (Math|Float|Lerp (LocalVariables|GetTargetArmLenght) (Variables|Default|GetTarget%20Arm%20Length) Alpha))
      (Transformation|SetRelativeRotation _springarmcomponent (Math|Rotator|Lerp(Rotator) (LocalVariables|GetRelativeRotation) (Variables|Default|GetNew%20Rotation) Alpha) false false))))