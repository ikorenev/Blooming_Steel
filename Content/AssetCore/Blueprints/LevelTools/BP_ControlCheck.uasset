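; BP_ControlCheck is a checkpoint volume that records where the player respawns and how movement and camera are oriented there.
; When the player overlaps its Box, it registers itself as the current control check on BP_MainGameMod.
; Respawn teleports the player to the Box and uses two arrows to set the movement plane constraint normal and WorldDirection.
; It also sets the spring arm's yaw from CameraAngle.
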(event OnComponentBeginOverlap(Box)
  (params (OverlappedComponent :type Primitive%20Component%20Object%20Reference) (OtherActor :type Actor%20Object%20Reference) (OtherComp :type Primitive%20Component%20Object%20Reference) (OtherBodyIndex :type Integer) (bFromSweep :type Boolean) (SweepResult :type Hit%20Result%20Structure%20%28by%20ref%29))
  (Utilities|Casting|CastToBP_Player OtherActor)
  (bind _asbp_main_game_mod (Utilities|Casting|CastToBP_MainGameMod (Game|GetGameMode)))
  (Variables|/Game/AssetCore/Blueprints/Core/BP_MainGameMod.BP_MainGameMod_C|SetCurrentControlCheck _asbp_main_game_mod self))

(event EventBeginPlay)

(event Collision|EventActorBeginOverlap
  (params (OtherActor :type Actor%20Object%20Reference)))

(event EventTick
  (params (DeltaSeconds :type Float%20%28single-precision%29)))

(fn ConstructionScript)

(fn Respawn
  (bind _returnvalue (Game|Player|GetPlayerPawn 0))
  (bind _asbp_player (Utilities|Casting|CastToBP_Player _returnvalue))
  (Transformation|SetActorLocation _returnvalue (Transformation|GetWorldLocation (Variables|Default|GetBox)) false true)
  (Class|MovementComponent|SetPlaneConstraintNormal (Variables|/Script/Engine.Character|GetCharacterMovement _asbp_player) (Math|Vector|GetForwardVector (Variables|Default|GetArrow1)))
  (Variables|/Game/AssetCore/Blueprints/Core/BP_Player.BP_Player_C|SetWorld%20Direction _asbp_player (Math|Vector|GetForwardVector (Variables|Default|GetArrow)))
  (Transformation|SetRelativeRotation (Variables|/Game/AssetCore/Blueprints/Core/BP_Player.BP_Player_C|GetSpringArm _asbp_player) (Math|Rotator|MakeRotator (.roll (Class|SpringArmComponent|GetTargetRotation (Variables|/Game/AssetCore/Blueprints/Core/BP_Player.BP_Player_C|GetSpringArm _asbp_player))) (.pitch (Class|SpringArmComponent|GetTargetRotation (Variables|/Game/AssetCore/Blueprints/Core/BP_Player.BP_Player_C|GetSpringArm _asbp_player))) (Variables|Default|GetCameraAngle)) false false))