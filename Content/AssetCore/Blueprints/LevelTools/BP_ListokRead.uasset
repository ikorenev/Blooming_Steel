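; Readable note actor that shows a full-screen Lists widget when the player interacts with it.
; Box overlap with BP_Player shows or hides the interact prompt through the HUD held by BP_MainGameMod.
; Each Interaction call flips between opening and removing the widget.
; While it is open, HUD_MainGame is hidden, move input is ignored and the player pawn is hidden, with the game left unpaused.
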(event OnComponentBeginOverlap(Box)
  (params (OverlappedComponent :type Primitive%20Component%20Object%20Reference) (OtherActor :type Actor%20Object%20Reference) (OtherComp :type Primitive%20Component%20Object%20Reference) (OtherBodyIndex :type Integer) (bFromSweep :type Boolean) (SweepResult :type Hit%20Result%20Structure%20%28by%20ref%29))
  (Utilities|Casting|CastToBP_Player OtherActor)
  ;[1 1 1] Включение подсказки, если ButtonRotate True
  (bind _asbp_main_game_mod (Utilities|Casting|CastToBP_MainGameMod (Game|GetGameMode)))
  (Default|InteractonDisplay (Variables|/Game/AssetCore/Blueprints/Core/BP_MainGameMod.BP_MainGameMod_C|GetHud _asbp_main_game_mod)))

(event OnComponentEndOverlap(Box)
  (params (OverlappedComponent :type Primitive%20Component%20Object%20Reference) (OtherActor :type Actor%20Object%20Reference) (OtherComp :type Primitive%20Component%20Object%20Reference) (OtherBodyIndex :type Integer))
  ;[1 1 1] Скрытие подсказки при выходе из тригера
  (Utilities|Casting|CastToBP_Player OtherActor)
  (bind _asbp_main_game_mod (Utilities|Casting|CastToBP_MainGameMod (Game|GetGameMode)))
  (Default|HideInteract (Variables|/Game/AssetCore/Blueprints/Core/BP_MainGameMod.BP_MainGameMod_C|GetHud _asbp_main_game_mod)))

(event EventBeginPlay)

(event Collision|EventActorBeginOverlap
  (params (OtherActor :type Actor%20Object%20Reference)))

(event EventTick
  (params (DeltaSeconds :type Float%20%28single-precision%29)))

(event EventInteraction
  (Utilities|FlowControl|FlipFlop
    (:A
      (bind _returnvalue (UserInterface|CreateWidget "/Game/AssetCore/UI/Lists.Lists_C"))
      (UserInterface|Viewport|AddtoViewport _returnvalue 0)
      (CallFunction|InitWidget))
    (:B
      (Widget|RemovefromParent _returnvalue)
      (CallFunction|EndWidget))))

(fn ConstructionScript)

(fn InitWidget
  (bind _returnvalue (Actor|GetActorOfClass "/Game/AssetCore/Blueprints/Core/HUD_MainGame.HUD_MainGame_C"))
  (Default|HideALL _returnvalue)
  (Input|SetIgnoreMoveInput (Game|GetPlayerController 0) true)
  (Game|SetGamePaused false)
  (Rendering|SetActorHiddenInGame (Game|Player|GetPlayerPawn 0) true))

(fn EndWidget
  (bind _returnvalue (Actor|GetActorOfClass "/Game/AssetCore/Blueprints/Core/HUD_MainGame.HUD_MainGame_C"))
  (Default|ShowAll _returnvalue)
  (Input|SetIgnoreMoveInput (Game|GetPlayerController 0) false)
  (Rendering|SetActorHiddenInGame (Game|Player|GetPlayerPawn 0) false))