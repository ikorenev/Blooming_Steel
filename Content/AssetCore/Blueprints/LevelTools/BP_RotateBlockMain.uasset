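; Trigger block that turns a plane-constrained player onto a new movement axis on overlap, or on interaction with a HUD prompt when IsButtonRotate is set.
; A gated toggle switches plane normal and WorldDirection between arrow-defined and first-stored values, with optional inversion.
; If IsRotateCamera is set, timelines swing the spring arm yaw by RotateAngle either way.
; The construction script optionally adds a collision box on a chosen side.
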(event OnComponentBeginOverlap(Box)
  (params (OverlappedComponent :type Primitive%20Component%20Object%20Reference) (OtherActor :type Actor%20Object%20Reference) (OtherComp :type Primitive%20Component%20Object%20Reference) (OtherBodyIndex :type Integer) (bFromSweep :type Boolean) (SweepResult :type Hit%20Result%20Structure%20%28by%20ref%29))
  (bind _arrow1 (Variables|Default|GetArrow1))
  (bind _returnvalue (Math|Vector|GetForwardVector _arrow1))
  ;[1 1 1] Вход в тригер
  (bind _asbp_player (Utilities|Casting|CastToBP_Player OtherActor))
  (Utilities|FlowControl|DoOnce false
    (:Completed
      (Utilities|FlowControl|Sequence
        (:then_0
          ;[1 1 1] Включение подсказки, если ButtonRotate True
          (if (Variables|Default|GetIsButtonRotate)
            (bind _asbp_main_game_mod (Utilities|Casting|CastToBP_MainGameMod (Game|GetGameMode)))
            (Default|InteractonDisplay (Variables|/Game/AssetCore/Blueprints/Core/BP_MainGameMod.BP_MainGameMod_C|GetHud _asbp_main_game_mod))
            (else
              ;[1 1 1] Включение поворота
              (Utilities|FlowControl|Sequence
                (:then_0
                  (goto _label Open))
                (:then_1
                  (Utilities|FlowControl|Gate true :!label _label
                    (:Exit
                      ;[1 1 1] Проверка направления блока и игрока
                      (Utilities|FlowControl|Sequence
                        (:then_0
                          ;[1 1 1] Запоминание прошлых координат игрока
                          (Utilities|FlowControl|DoOnce false
                            (:Completed
                              (Variables|Default|SetLast%20Forward (Transformation|GetActorForwardVector _asbp_player))
                              (Variables|Default|SetLastNormal (Class|MovementComponent|GetPlaneConstraintNormal (Variables|/Script/Engine.Character|GetCharacterMovement _asbp_player))))))
                        (:then_1
                          (if (Utilities|Operators|EqualEqual (Class|MovementComponent|GetPlaneConstraintNormal (Variables|/Script/Engine.Character|GetCharacterMovement _asbp_player)) (Variables|Default|GetLastNormal) 0.01)
                            ;[1 1 1] Если новое направление не равно, тому что было у игрока задать новое
                            (Class|MovementComponent|SetPlaneConstraintNormal (Variables|/Script/Engine.Character|GetCharacterMovement _asbp_player) (Math|Vector|GetForwardVector (Variables|Default|GetArrow)))
                            (if (Variables|Default|GetIsInveriveController)
                              (Variables|/Game/AssetCore/Blueprints/BattleSystem/CharactersClass/BP_Player.BP_Player_C|SetWorld%20Direction _asbp_player (* _returnvalue -1.0))
                              (else
                                (Variables|/Game/AssetCore/Blueprints/BattleSystem/CharactersClass/BP_Player.BP_Player_C|SetWorld%20Direction _asbp_player _returnvalue)))
                            (Variables|Default|SetNewCameraRotate true)
                            (else
                              ;[1 1 1] Возврат игрока на прошлую траекторию
                              (Class|MovementComponent|SetPlaneConstraintNormal (Variables|/Script/Engine.Character|GetCharacterMovement _asbp_player) (Variables|Default|GetLastNormal))
                              (if (Variables|Default|GetIsSecondInvertController)
                                (Variables|/Game/AssetCore/Blueprints/BattleSystem/CharactersClass/BP_Player.BP_Player_C|SetWorld%20Direction _asbp_player (* (Variables|Default|GetLast%20Forward) -1.0))
                                (else
                                  (Variables|/Game/AssetCore/Blueprints/BattleSystem/CharactersClass/BP_Player.BP_Player_C|SetWorld%20Direction _asbp_player (Variables|Default|GetLast%20Forward))))
                              (Variables|Default|SetNewCameraRotate false))))
                        (:then_2
                          (if (Variables|Default|GetIsRotateCamera)
                            (Utilities|FlowControl|DoOnce false :!label _label_2
                              (:Completed
                                (if (Variables|Default|GetNewCameraRotate)
                                  ;[1 1 1] Поворот камеры игрока
                                  (Variables|Default|SetReturn%20Value%20Z%20%28Yaw%29 (.yaw (Transformation|GetSocketRotation (Variables|/Game/AssetCore/Blueprints/BattleSystem/CharactersClass/BP_Player.BP_Player_C|GetSpringArm _asbp_player) "None")))
                                  (bind _newtrack_0 (Timeline|Timeline_0 PlayFromStart)
                                    (:Update
                                      (Transformation|SetRelativeRotation (Variables|/Game/AssetCore/Blueprints/BattleSystem/CharactersClass/BP_Player.BP_Player_C|GetSpringArm _asbp_player) (Math|Rotator|MakeRotator (.roll (Class|SpringArmComponent|GetTargetRotation (Variables|/Game/AssetCore/Blueprints/BattleSystem/CharactersClass/BP_Player.BP_Player_C|GetSpringArm _asbp_player))) (.pitch (Class|SpringArmComponent|GetTargetRotation (Variables|/Game/AssetCore/Blueprints/BattleSystem/CharactersClass/BP_Player.BP_Player_C|GetSpringArm _asbp_player))) (Math|Float|Lerp (Variables|Default|GetReturn%20Value%20Z%20%28Yaw%29) (+ (Variables|Default|GetReturn%20Value%20Z%20%28Yaw%29) (Variables|Default|GetRotateAngle)) _newtrack_0)) false false))
                                    (:Finished
                                      (goto _label_2 Reset)))
                                  (else
                                    ;[1 1 1] Возращение камеры обратно
                                    (Variables|Default|SetReturn%20Value%20Z%20%28Yaw%29 (.yaw (Transformation|GetSocketRotation (Variables|/Game/AssetCore/Blueprints/BattleSystem/CharactersClass/BP_Player.BP_Player_C|GetSpringArm _asbp_player) "None")))
                                    (bind _newtrack_0_2 (Timeline|Timeline_1 PlayFromStart)
                                      (:Update
                                        (Transformation|SetRelativeRotation (Variables|/Game/AssetCore/Blueprints/BattleSystem/CharactersClass/BP_Player.BP_Player_C|GetSpringArm _asbp_player) (Math|Rotator|MakeRotator (.roll (Class|SpringArmComponent|GetTargetRotation (Variables|/Game/AssetCore/Blueprints/BattleSystem/CharactersClass/BP_Player.BP_Player_C|GetSpringArm _asbp_player))) (.pitch (Class|SpringArmComponent|GetTargetRotation (Variables|/Game/AssetCore/Blueprints/BattleSystem/CharactersClass/BP_Player.BP_Player_C|GetSpringArm _asbp_player))) (Math|Float|Lerp (Variables|Default|GetReturn%20Value%20Z%20%28Yaw%29) (- (Variables|Default|GetReturn%20Value%20Z%20%28Yaw%29) (Variables|Default|GetRotateAngle)) _newtrack_0_2)) false false))
                                      (:Finished
                                        (goto _label_2 Reset)))))))))))))))))
        (:then_1
          (Utilities|Time|SetTimerbyEvent (delegate Custom|Reset) 0.1))))))

(event OnComponentEndOverlap(Box)
  (params (OverlappedComponent :type Primitive%20Component%20Object%20Reference) (OtherActor :type Actor%20Object%20Reference) (OtherComp :type Primitive%20Component%20Object%20Reference) (OtherBodyIndex :type Integer))
  ;[1 1 1] Скрытие подсказки при выходе из тригера
  (Utilities|Casting|CastToBP_Player OtherActor)
  (bind _asbp_main_game_mod (Utilities|Casting|CastToBP_MainGameMod (Game|GetGameMode)))
  (Default|HideInteract (Variables|/Game/AssetCore/Blueprints/Core/BP_MainGameMod.BP_MainGameMod_C|GetHud _asbp_main_game_mod)))

(event Custom|CustomEvent
  (params (OverlappedComponent :type Primitive%20Component%20Object%20Reference) (OtherActor :type Actor%20Object%20Reference) (OtherComp :type Primitive%20Component%20Object%20Reference) (OtherBodyIndex :type Integer)))

(event Custom|Reset
  (bind _arrow1 (Variables|Default|GetArrow1))
  (bind _returnvalue (Math|Vector|GetForwardVector _arrow1))
  (Utilities|FlowControl|DoOnce false) ; enters at Reset
)

(event EventBeginPlay)

(event Collision|EventActorBeginOverlap
  (params (OtherActor :type Actor%20Object%20Reference)))

(event EventInteraction
  (bind _arrow1 (Variables|Default|GetArrow1))
  (bind _returnvalue (Math|Vector|GetForwardVector _arrow1))
  ;[1 1 1] Включение поворота
  (Utilities|FlowControl|Sequence
    (:then_0
      (goto _label Open))
    (:then_1
      (Utilities|FlowControl|Gate true :!label _label
        (:Exit
          ;[1 1 1] Проверка направления блока и игрока
          (Utilities|FlowControl|Sequence
            (:then_0
              ;[1 1 1] Запоминание прошлых координат игрока
              (Utilities|FlowControl|DoOnce false
                (:Completed
                  (Variables|Default|SetLast%20Forward (Transformation|GetActorForwardVector (stale OnComponentBeginOverlap(Box) _asbp_player)))
                  (Variables|Default|SetLastNormal (Class|MovementComponent|GetPlaneConstraintNormal (Variables|/Script/Engine.Character|GetCharacterMovement (stale OnComponentBeginOverlap(Box) _asbp_player)))))))
            (:then_1
              (if (Utilities|Operators|EqualEqual (Class|MovementComponent|GetPlaneConstraintNormal (Variables|/Script/Engine.Character|GetCharacterMovement (stale OnComponentBeginOverlap(Box) _asbp_player))) (Variables|Default|GetLastNormal) 0.01)
                ;[1 1 1] Если новое направление не равно, тому что было у игрока задать новое
                (Class|MovementComponent|SetPlaneConstraintNormal (Variables|/Script/Engine.Character|GetCharacterMovement (stale OnComponentBeginOverlap(Box) _asbp_player)) (Math|Vector|GetForwardVector (Variables|Default|GetArrow)))
                (if (Variables|Default|GetIsInveriveController)
                  (Variables|/Game/AssetCore/Blueprints/BattleSystem/CharactersClass/BP_Player.BP_Player_C|SetWorld%20Direction (stale OnComponentBeginOverlap(Box) _asbp_player) (* _returnvalue -1.0))
                  (else
                    (Variables|/Game/AssetCore/Blueprints/BattleSystem/CharactersClass/BP_Player.BP_Player_C|SetWorld%20Direction (stale OnComponentBeginOverlap(Box) _asbp_player) _returnvalue)))
                (Variables|Default|SetNewCameraRotate true)
                (else
                  ;[1 1 1] Возврат игрока на прошлую траекторию
                  (Class|MovementComponent|SetPlaneConstraintNormal (Variables|/Script/Engine.Character|GetCharacterMovement (stale OnComponentBeginOverlap(Box) _asbp_player)) (Variables|Default|GetLastNormal))
                  (if (Variables|Default|GetIsSecondInvertController)
                    (Variables|/Game/AssetCore/Blueprints/BattleSystem/CharactersClass/BP_Player.BP_Player_C|SetWorld%20Direction (stale OnComponentBeginOverlap(Box) _asbp_player) (* (Variables|Default|GetLast%20Forward) -1.0))
                    (else
                      (Variables|/Game/AssetCore/Blueprints/BattleSystem/CharactersClass/BP_Player.BP_Player_C|SetWorld%20Direction (stale OnComponentBeginOverlap(Box) _asbp_player) (Variables|Default|GetLast%20Forward))))
                  (Variables|Default|SetNewCameraRotate false))))
            (:then_2
              (if (Variables|Default|GetIsRotateCamera)
                (Utilities|FlowControl|DoOnce false :!label _label_2
                  (:Completed
                    (if (Variables|Default|GetNewCameraRotate)
                      ;[1 1 1] Поворот камеры игрока
                      (Variables|Default|SetReturn%20Value%20Z%20%28Yaw%29 (.yaw (Transformation|GetSocketRotation (Variables|/Game/AssetCore/Blueprints/BattleSystem/CharactersClass/BP_Player.BP_Player_C|GetSpringArm (stale OnComponentBeginOverlap(Box) _asbp_player)) "None")))
                      (bind _newtrack_0 (Timeline|Timeline_0 PlayFromStart)
                        (:Update
                          (Transformation|SetRelativeRotation (Variables|/Game/AssetCore/Blueprints/BattleSystem/CharactersClass/BP_Player.BP_Player_C|GetSpringArm (stale OnComponentBeginOverlap(Box) _asbp_player)) (Math|Rotator|MakeRotator (.roll (Class|SpringArmComponent|GetTargetRotation (Variables|/Game/AssetCore/Blueprints/BattleSystem/CharactersClass/BP_Player.BP_Player_C|GetSpringArm (stale OnComponentBeginOverlap(Box) _asbp_player)))) (.pitch (Class|SpringArmComponent|GetTargetRotation (Variables|/Game/AssetCore/Blueprints/BattleSystem/CharactersClass/BP_Player.BP_Player_C|GetSpringArm (stale OnComponentBeginOverlap(Box) _asbp_player)))) (Math|Float|Lerp (Variables|Default|GetReturn%20Value%20Z%20%28Yaw%29) (+ (Variables|Default|GetReturn%20Value%20Z%20%28Yaw%29) (Variables|Default|GetRotateAngle)) _newtrack_0)) false false))
                        (:Finished
                          (goto _label_2 Reset)))
                      (else
                        ;[1 1 1] Возращение камеры обратно
                        (Variables|Default|SetReturn%20Value%20Z%20%28Yaw%29 (.yaw (Transformation|GetSocketRotation (Variables|/Game/AssetCore/Blueprints/BattleSystem/CharactersClass/BP_Player.BP_Player_C|GetSpringArm (stale OnComponentBeginOverlap(Box) _asbp_player)) "None")))
                        (bind _newtrack_0_2 (Timeline|Timeline_1 PlayFromStart)
                          (:Update
                            (Transformation|SetRelativeRotation (Variables|/Game/AssetCore/Blueprints/BattleSystem/CharactersClass/BP_Player.BP_Player_C|GetSpringArm (stale OnComponentBeginOverlap(Box) _asbp_player)) (Math|Rotator|MakeRotator (.roll (Class|SpringArmComponent|GetTargetRotation (Variables|/Game/AssetCore/Blueprints/BattleSystem/CharactersClass/BP_Player.BP_Player_C|GetSpringArm (stale OnComponentBeginOverlap(Box) _asbp_player)))) (.pitch (Class|SpringArmComponent|GetTargetRotation (Variables|/Game/AssetCore/Blueprints/BattleSystem/CharactersClass/BP_Player.BP_Player_C|GetSpringArm (stale OnComponentBeginOverlap(Box) _asbp_player)))) (Math|Float|Lerp (Variables|Default|GetReturn%20Value%20Z%20%28Yaw%29) (- (Variables|Default|GetReturn%20Value%20Z%20%28Yaw%29) (Variables|Default|GetRotateAngle)) _newtrack_0_2)) false false))
                          (:Finished
                            (goto _label_2 Reset)))))))))))))))

(fn ConstructionScript
  (if (Variables|Default|GetNeed%20Collision)
    (switch Utilities|FlowControl|Switch|SwitchonBoxCollisions (Variables|Default|GetNewVar)
      (:NewEnumerator0
        (AddComponent|AddBoxComponent false (Math|Transform|MakeTransform "60.000000,0.000000,0.000000" "0.000000,-90.000000,0.000000" "1.000000,1.000000,1.000000")))
      (:NewEnumerator1
        (AddComponent|AddBoxComponent false (Math|Transform|MakeTransform "-60.000000,0.000000,0.000000" "0.000000,90.000000,0.000000" "2.400000,0.330000,1.000000")))
      (:NewEnumerator2
        (AddComponent|AddBoxComponent false (Math|Transform|MakeTransform "0.000000,60.000000,0.000000" "0, 0, 0" "1.000000,1.000000,1.000000")))
      (:NewEnumerator3
        (AddComponent|AddBoxComponent false (Math|Transform|MakeTransform "0.000000,-47.000000,0.000000" "0, 0, 0" "1.000000,0.500000,1.000000"))))))

(fn CalculateCamera
  (params (self2 :type BP%20Player%20Object%20Reference)))