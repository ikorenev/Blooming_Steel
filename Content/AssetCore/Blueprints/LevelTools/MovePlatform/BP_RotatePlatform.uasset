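; BP_RotatePlatform is a level platform that rotates back and forth between a start and end rotation.
; BeginPlay starts a looping timer spaced by travel time plus pause, with a negative start delay offsetting the first interval.
; Each tick of that timer flip-flops a timeline between play and reverse, lerping the mesh's relative rotation.
; The construction script sets the timeline play rate from SpeedRate and derives travel time as its inverse.
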(event Custom|Trigger
  (Utilities|FlowControl|FlipFlop
    (:A
      (bind _newtrack_0 (Timeline|PatrulLine Play)
        (:Update
          (Transformation|SetRelativeRotation (Variables|Default|GetStaticMesh) (Math|Rotator|Lerp(Rotator) (Variables|Default|GetStartRotation) (Variables|Default|GetEndRotation) _newtrack_0) false false))))
    (:B
      (Timeline|PatrulLine Reverse))))

(event EventBeginPlay
  (bind _time_length (Variables|Default|GetTime%20Length))
  (bind _timepause (Variables|Default|GetTimePause))
  (bind _returnvalue (+ _time_length _timepause))
  (Utilities|Time|SetTimerbyEvent (delegate Custom|Trigger) _returnvalue true (* _returnvalue -1.0)))

(event Collision|EventActorBeginOverlap
  (params (OtherActor :type Actor%20Object%20Reference)))

(event EventTick
  (params (DeltaSeconds :type Float%20%28single-precision%29)))

(fn ConstructionScript
  (bind _speedrate (Variables|Default|GetSpeedRate))
  (Components|Timeline|SetPlayRate (Variables|Default|GetPatrulLine) _speedrate)
  (Variables|Default|SetTime%20Length (/ 1.0 _speedrate)))