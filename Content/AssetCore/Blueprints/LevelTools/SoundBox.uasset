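; SoundBox is a level-tool actor that plays an assignable sound while BP_Player is inside its box.
; The construction script sets the sound on an AudioCurveSource, and a looping timer, offset to fire immediately, polls the box overlaps.
; While occupied, each check restarts playback at a counter-based offset and increments the counter; otherwise it pauses.
; The counter never resets, so re-entry continues from the accumulated position.
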(event Custom|CheckPlayer
  (bind _audiocurvesource (Variables|Default|GetAudioCurveSource))
  (bind _newvar (Variables|Default|GetNewVar))
  (if (Utilities|Array|IsNotEmpty (Collision|GetOverlappingActors (Variables|Default|GetBox) "/Game/AssetCore/Blueprints/BattleSystem/CharactersClass/BP_Player.BP_Player_C" :!class /Script/Engine.PrimitiveComponent))
    (Audio|Components|Audio|Play _audiocurvesource (* (Variables|Default|GetTime) _newvar))
    (Math|Float|IncrementFloat _newvar)
    (else
      (Class|AudioComponent|SetPaused _audiocurvesource true))))

(event EventBeginPlay
  (bind _time (Variables|Default|GetTime))
  (Utilities|Time|SetTimerbyEvent (delegate Custom|CheckPlayer) _time true (* _time -1.0)))

(event Collision|EventActorBeginOverlap
  (params (OtherActor :type Actor%20Object%20Reference)))

(event EventTick
  (params (DeltaSeconds :type Float%20%28single-precision%29)))

(fn ConstructionScript
  (Audio|Components|Audio|SetSound (Variables|Default|GetAudioCurveSource) (Variables|Default|GetNew%20Sound)))