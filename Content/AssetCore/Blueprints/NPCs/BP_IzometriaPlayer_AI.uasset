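; Isometric hero character, named as an AI variant of the player, with world-axis movement, sprint, and hit and death montages.
; The Interact input messages every actor overlapping the capsule, a workaround the author flags as a hack.
; ActiveHero starts a looping timer for a forward box trace whose result is unused, and DeactiveHero pauses it.
; BeginPlay, WASD handlers and InitChars are empty stubs, and the respawn binding never runs.
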(event Custom|Hit%20Animation
  (Animation|Montage|PlayMontage (Variables|Character|GetMesh) (Utilities|Select :Index (Math|Random|RandomInteger 2) :Option%200 (Variables|Default|GetAnimMontage1) :Option%201 (Variables|Default|GetAnimMontage2))))

(event Custom|Respawn
  (CallFunction|InitChars))

(event Custom|Change%20death
  (Animation|Montage|PlayMontage (Variables|Character|GetMesh) "/Game/AssetCore/Blueprints/Animation/Standing_Death_Backward_01__1__Montage.Standing_Death_Backward_01__1__Montage"
    (:OnCompleted
      (Utilities|FlowControl|Delay 0.02))))

(event Custom|MoveSide
  (params (Axis :type Float%20%28double-precision%29))
  (Pawn|Input|AddMovementInput "0.000000,1.000000,0.000000" Axis false))

(event Custom|Move%20Front
  (params (Axis :type Float%20%28double-precision%29))
  (Pawn|Input|AddMovementInput "1.000000,0.000000,0.000000" Axis false))

(event Custom|ActiveHero
  (bind _returnvalue (Utilities|Time|SetTimerbyEvent (delegate Custom|Interact) 0.05 true))
  (Variables|Default|SetisActive? true))

(event Custom|Interact
  (bind _returnvalue (Transformation|GetActorLocation))
  (Collision|BoxTraceByChannel _returnvalue (+ _returnvalue (* (Transformation|GetActorForwardVector) 8e+01)) "50.000000,50.000000,50.000000" "0, 0, 0" "TraceTypeQuery1" false 0 "None"))

(event Custom|DeactiveHero
  (if (Utilities|Time|IsValidTimerHandle (stale Custom|ActiveHero _returnvalue))
    (Utilities|Time|PauseTimerbyHandle (stale Custom|ActiveHero _returnvalue))
    (Variables|Default|SetisActive? false)))

(event EventBeginPlay)

(event Input|ActionEvents|InputActionSprint
  (params (Key :type Key%20Structure))
  (bind _charactermovement (Variables|Character|GetCharacterMovement))
  (:Pressed
    (Variables|/Script/Engine.CharacterMovementComponent|SetMaxWalkSpeed _charactermovement 8e+02))
  (:Released
    (Variables|/Script/Engine.CharacterMovementComponent|SetMaxWalkSpeed _charactermovement 4e+02)))

(event Input|ActionEvents|InputActionInteract
  (params (Key :type Key%20Structure))
  ;[1 1 1] Интерактивность(Внимание костыль)
  (:Pressed
    (for _array_element (Collision|GetOverlappingActors (Variables|Collision|GetCapsuleComponent) 0 :!class /Script/Engine.PrimitiveComponent)
      (Class|Interaction|Interaction(Message) _array_element))))

(event Input|KeyboardEvents|W
  (params (Key :type Key%20Structure))
  (:Pressed
    (if true
      _)))

(event Input|KeyboardEvents|A
  (params (Key :type Key%20Structure))
  (:Pressed
    (if true
      _)))

(event Input|KeyboardEvents|S
  (params (Key :type Key%20Structure))
  (:Pressed
    (if true
      _)))

(event Input|KeyboardEvents|D
  (params (Key :type Key%20Structure))
  (:Pressed
    (if true
      _)))

(fn ConstructionScript)

(fn InitChars)