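; Player character for animation testing, with crouch, sprint, rotate-block interaction, a camera height toggle and ledge hanging.
; Jumping runs a timed capsule-trace loop that snaps the capsule onto a hit physics-body hold and disables movement.
; While hanging, WASD box-traces for the next hold, storing hand socket locations; F, or a missed up/down trace, restores walking.
; Simple setters expose movement state flags; hero-switching functions are empty stubs.
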(event EventBeginPlay)

(event Collision|EventActorBeginOverlap
  (params (OtherActor :type Actor%20Object%20Reference)))

(event Input|ActionEvents|InputActionSprint
  (params (Key :type Key%20Structure :default "None"))
  (bind _charactermovement (Variables|Character|GetCharacterMovement))
  (:Pressed
    (Variables|/Script/Engine.CharacterMovementComponent|SetMaxWalkSpeed _charactermovement 8e+02))
  (:Released
    (Variables|/Script/Engine.CharacterMovementComponent|SetMaxWalkSpeed _charactermovement 4e+02)))

(event Input|ActionEvents|InputActionJump
  (params (Key :type Key%20Structure :default "None"))
  (bind _self self)
  (bind _capsulecomponent (Variables|Collision|GetCapsuleComponent))
  (bind _returnvalue (Transformation|GetActorLocation _self))
  (:Pressed
    (if (not (Variables|Default|GetHoop))
      (Character|Jump)
      (Default|CallJumpDispathcer)
      (Utilities|LoopDelay 0.1 :!label _label
        (:Complete
          (if (Variables|Default|GetHoop)
            (Utilities|Array|Add (Utilities|Array|MakeArray 0) (.HitActor (Collision|BreakHitResult (stale _outhit))))
            (Components|MoveComponentTo _capsulecomponent (Math|Vector|MakeVector (.X (Math|Vector|BreakVector (.Location (Collision|BreakHitResult (stale _outhit))))) (.Y (Math|Vector|BreakVector (.Location (Collision|BreakHitResult (stale _outhit))))) (- (.z (Transformation|GetWorldLocation (.HitComponent (Collision|BreakHitResult (stale _outhit))))) 8e+01)) (Math|Rotator|MakeRotator 0.0 0.0 (+ (.yaw (Math|Conversions|RotationFromXVector (.Normal (Collision|BreakHitResult (stale _outhit))))) 1.8e+02)) false false 0.2 false)
            (Variables|Default|SetArray%20to%20ignore (Utilities|Array|MakeArray (.HitActor (Collision|BreakHitResult (stale _outhit)))))
            (Transformation|AddLocalOffset _capsulecomponent "10.000000, 0,-25.000000" false false)
            (Pawn|Components|CharacterMovement|SetMovementMode (Variables|Character|GetCharacterMovement) "MOVE_None" 0)
            (Variables|Default|SetRight%20 (Transformation|GetSocketLocation (.HitComponent (Collision|BreakHitResult (stale _outhit))) "SocketR"))
            (Variables|Default|SetLeft%20 (Transformation|GetSocketLocation (.HitComponent (Collision|BreakHitResult (stale _outhit))) "SocketL"))))
        (:Body
          (bind (_outhit _returnvalue_2) (Class|KismetSystemLibrary|CapsuleTraceSingleforObjects _returnvalue (+ _returnvalue (* (Transformation|GetActorForwardVector _self) 50)) 6e+01 1.2e+02 (Utilities|Array|MakeArray "ObjectTypeQuery4") false 0 "None" true))
          (if _returnvalue_2
            (Variables|Default|SetHoop true)
            (goto _label Break))))))
  (:Released
    (Character|StopJumping)
    (CallFunction|ChangeJump false)
    (if (Utilities|Enum|NotEqual(Enum) (Variables|/Script/Engine.CharacterMovementComponent|GetMovementMode (Variables|Character|GetCharacterMovement)) "MOVE_None") :!label _label_2
      (goto _label Break)
      (else
        (Utilities|FlowControl|Delay 0.05)
        (goto _label_2)))))

(event Input|ActionEvents|InputActionCrouch
  (params (Key :type Key%20Structure :default "None"))
  (:Pressed
    (CallFunction|ChangeCrouch true)
    (Character|Crouch))
  (:Released
    (CallFunction|ChangeCrouch false)
    (Character|UnCrouch)))

(event Input|ActionEvents|InputActionLoockDown
  (params (Key :type Key%20Structure :default "None"))
  (bind _camera (Variables|Default|GetCamera))
  (bind _camera_2 (Variables|Default|GetCamera))
  (bind _relativelocation (Variables|/Script/Engine.SceneComponent|GetRelativeLocation _camera))
  (bind _relativelocation_2 (Variables|/Script/Engine.SceneComponent|GetRelativeLocation _camera_2))
  (:Pressed
    (Utilities|FlowControl|FlipFlop
      (:A
        (bind _newtrack_0 (Timeline|Timeline_0 PlayFromStart)
          (:Update
            (Transformation|SetRelativeLocation _camera_2 (Math|Vector|MakeVector (.x _relativelocation_2) (.y _relativelocation_2) (+ (.z _relativelocation_2) (Math|Float|Lerp 0.0 -12.0 _newtrack_0))) false false))))
      (:B
        (bind _newtrack_0_2 (Timeline|Timeline_1 PlayFromStart)
          (:Update
            (Transformation|SetRelativeLocation _camera (Math|Vector|MakeVector (.x _relativelocation) (.y _relativelocation) (+ (.z _relativelocation) (Math|Float|Lerp 0.0 12.0 _newtrack_0_2))) false false)))))))

(event Input|ActionEvents|InputActionInteract
  (params (Key :type Key%20Structure :default "None"))
  (:Pressed
    (for _array_element (Collision|GetOverlappingActors (Variables|Collision|GetCapsuleComponent) "/Game/Blueprints/LevelTools/BP_RotateBlock.BP_RotateBlock_C" :!class /Script/Engine.PrimitiveComponent)
      (Class|Interact|Interaction(Message) _array_element))))

(event Input|AxisEvents|InputAxisMoveForward/Backward
  (params (AxisValue :type Float%20%28single-precision%29))
  (Pawn|Input|AddMovementInput (Variables|Default|GetWorld%20Direction) AxisValue false))

(event Input|KeyboardEvents|W
  (params (Key :type Key%20Structure :default "None"))
  (:Pressed
    (CallFunction|ChangeIdle true)
    (if (Variables|Default|GetHoop)
      (Utilities|HoopTrace (Variables|Default|GetTrace) "NewEnumerator0")))
  (:Released
    (CallFunction|ChangeIdle false)))

(event Input|KeyboardEvents|A
  (params (Key :type Key%20Structure :default "None"))
  (:Pressed
    (CallFunction|ChangeIdle true)
    (if (Variables|Default|GetHoop)
      (Utilities|HoopTrace (Variables|Default|GetTrace) "NewEnumerator3")))
  (:Released
    (CallFunction|ChangeIdle false)))

(event Input|KeyboardEvents|S
  (params (Key :type Key%20Structure :default "None"))
  (:Pressed
    (CallFunction|ChangeIdle true)
    (if (Variables|Default|GetHoop)
      (Utilities|HoopTrace (Variables|Default|GetTrace) "NewEnumerator1")))
  (:Released
    (CallFunction|ChangeIdle false)))

(event Input|KeyboardEvents|D
  (params (Key :type Key%20Structure :default "None"))
  (:Pressed
    (CallFunction|ChangeIdle true)
    (if (Variables|Default|GetHoop)
      (Utilities|HoopTrace (Variables|Default|GetTrace) "NewEnumerator2")))
  (:Released
    (CallFunction|ChangeIdle false)))

(event Input|KeyboardEvents|F
  (params (Key :type Key%20Structure :default "None"))
  (:Pressed
    (if (Variables|Default|GetHoop)
      (Variables|Default|SetHoop false)
      (Pawn|Components|CharacterMovement|SetMovementMode (Variables|Character|GetCharacterMovement) "MOVE_Walking" 0))))

(fn ConstructionScript)

(fn ChangeHero
  (params (HeroSlot :type Integer)))

(fn InitChars)

(fn GetCurrentHero)

(fn ChangeIdle
  (params (isPressed :type Boolean))
  (Variables|Default|SetSpeed isPressed))

(fn ChangeCrouch
  (params (isCrouching :type Boolean))
  (Variables|Default|SetCrouching isCrouching))

(fn ChangeJump
  (params (Jumping :type Boolean))
  (Variables|Default|SetJumping Jumping))