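; BP_PlayerController is a player controller that handles hero switching and party selection input.
; Four hero actions set a slot index and call ChangeHero on the player's BP_Player character.
; The SelectParty action flip-flops between streaming in the ChangeHero level with CallSetParty and unloading it with CallReturnGame.
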(event EventBeginPlay)

(event EventTick
  (params (DeltaSeconds :type Float%20%28single-precision%29)))

(event Input|ActionEvents|InputActionHero1
  (params (Key :type Key%20Structure :default "None"))
  (:Pressed
    (Variables|Default|SetHero%20Slot 0)
    (bind _asbp_player (Utilities|Casting|CastToBP_Player (Game|GetPlayerCharacter 0)))
    (Default|ChangeHero _asbp_player (Variables|Default|GetHero%20Slot))))

(event Input|ActionEvents|InputActionHero2
  (params (Key :type Key%20Structure :default "None"))
  (:Pressed
    (Variables|Default|SetHero%20Slot 1)
    (bind _asbp_player (Utilities|Casting|CastToBP_Player (Game|GetPlayerCharacter 0)))
    (Default|ChangeHero _asbp_player (Variables|Default|GetHero%20Slot))))

(event Input|ActionEvents|InputActionHero3
  (params (Key :type Key%20Structure :default "None"))
  (:Pressed
    (Variables|Default|SetHero%20Slot 2)
    (bind _asbp_player (Utilities|Casting|CastToBP_Player (Game|GetPlayerCharacter 0)))
    (Default|ChangeHero _asbp_player (Variables|Default|GetHero%20Slot))))

(event Input|ActionEvents|InputActionHero4
  (params (Key :type Key%20Structure :default "None"))
  (:Pressed
    (Variables|Default|SetHero%20Slot 3)
    (bind _asbp_player (Utilities|Casting|CastToBP_Player (Game|GetPlayerCharacter 0)))
    (Default|ChangeHero _asbp_player (Variables|Default|GetHero%20Slot))))

(event Input|ActionEvents|InputActionSelectParty
  (params (Key :type Key%20Structure :default "None"))
  (:Pressed
    (Utilities|FlowControl|FlipFlop
      (:A
        (Class|GameplayStatics|LoadStreamLevelbySoftObjectPtr "/Game/Maps/ChangeHero.ChangeHero" true false)
        (Default|CallSetParty))
      (:B
        (Class|GameplayStatics|UnloadStreamLevelbySoftObjectPtr "/Game/Maps/ChangeHero.ChangeHero" false)
        (Default|CallReturnGame)))))

(fn ConstructionScript)