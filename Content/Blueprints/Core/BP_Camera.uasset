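; BP_Camera spawns a separate camera actor, makes it the player's view target and keeps it at a fixed world offset from the player pawn each Tick.
; A looping timer runs CameraHide, which box-traces from camera to pawn on the Visibility channel and hides the root component of any StaticMeshActor hit.
; Hidden meshes stay hidden, since the re-show logic is disconnected, as are the spring arm nodes.
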(event Custom|CameraHide
  (bind _outhits (Class|KismetSystemLibrary|BoxTraceMulti (Transformation|GetWorldLocation (Variables|/Script/Engine.Actor|GetRootComponent (stale EventBeginPlay _returnvalue))) (Transformation|GetActorLocation (Game|Player|GetPlayerPawn 0)) "80.000000,80.000000,200.000000" "0, 0, 0" "TraceTypeQuery1" false 0 "None" true))
  (for _array_element _outhits
    (if true
      (Utilities|FlowControl|Sequence
        (:then_1
          (bind _asstatic_mesh_actor (Utilities|Casting|CastToStaticMeshActor (.HitActor (Collision|BreakHitResult _array_element))))
          (bind _output_get (Variables|Default|SetHideActor _asstatic_mesh_actor))
          (Rendering|SetVisibility (Variables|/Script/Engine.Actor|GetRootComponent _output_get) false false))))))

(event EventBeginPlay
  (bind _returnvalue (Game|SpawnActorfromClass "/Script/Engine.CameraActor" (Math|Transform|MakeTransform "0, 0, 0" "0, 0, 0" "1.000000,1.000000,1.000000") "Undefined" 0 0))
  (Variables|Default|SetCameraActor _returnvalue)
  (Game|Player|SetViewTargetwithBlend (Game|GetPlayerController 0) _returnvalue 0.0 "VTBlend_Linear" 0.0 false)
  (Utilities|Time|SetTimerbyFunctionName 0 "CameraHide" 0.2 true -0.2))

(event Collision|EventActorBeginOverlap
  (params (OtherActor :type Actor%20Object%20Reference)))

(event EventTick
  (params (DeltaSeconds :type Float%20%28single-precision%29))
  (Transformation|SetWorldLocation (Variables|/Script/Engine.Actor|GetRootComponent (stale EventBeginPlay _returnvalue)) (+ (Transformation|GetActorLocation (Game|Player|GetPlayerPawn 0)) "-500.000000,0.000000,200.000000") false false))

(fn ConstructionScript)