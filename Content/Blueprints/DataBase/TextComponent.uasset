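; TextComponent is a component that passes multi-page text to its TextUnderHead widget, apparently dialogue shown at a character.
; SetText124 formats each array entry with a supplied pattern, appends the results into one text and hands it to the widget with min/max auto-page intervals.
; It then sets the widget's page count to the array length and forces EndDelay to zero, ignoring the EndDelay input.
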(event EventBeginPlay)

(event EventTick
  (params (DeltaSeconds :type Float%20%28single-precision%29)))

(fn SetText124
  (params (NewParam :type Text) (Auto%20Next%20Dialogue%20Msg%20Page%20Interval%20Min :type Float%20%28double-precision%29) (Auto%20Next%20Dialogue%20Msg%20Page%20Interval%20Max :type Float%20%28double-precision%29) (ArrayText :type Array%20of%20Strings) (EndDelay :type Float%20%28double-precision%29))
  (for _array_element ArrayText
    (Variables|Default|SetFinalyText (Utilities|String|Append (Variables|Default|GetFinalyText) (Utilities|String|ToString(Text) (Utilities|Text|FormatText NewParam _array_element)))))
  (bind _astext_under_head (Utilities|Casting|CastToTextUnderHead (UserInterface|GetWidget)))
  (Default|SetText _astext_under_head Auto%20Next%20Dialogue%20Msg%20Page%20Interval%20Min Auto%20Next%20Dialogue%20Msg%20Page%20Interval%20Max (Utilities|Text|ToText(String) (Variables|Default|GetFinalyText)))
  (Variables|/Game/UI/TextUnderHead.TextUnderHead_C|SetPages _astext_under_head (Utilities|Array|Length ArrayText))
  (Variables|/Game/UI/TextUnderHead.TextUnderHead_C|SetEndDelay _astext_under_head 0.0))