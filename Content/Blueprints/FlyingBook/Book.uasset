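; Flying book actor that travels along the spline of a SplineBook actor found in the level at BeginPlay.
; Each tick a BP_Player overlaps its Box, it picks one of three speeds from the player's signed world Y offset to the book.
; MoveObject advances the clamped spline distance by that per-frame step, without delta-time scaling, and sets location and rotation from the spline.
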(event Custom|Move%20Object
  (bind _splineref (Variables|Default|GetSplineRef))
  (bind _spline (Variables|/Game/Blueprints/FlyingBook/SplineBook.SplineBook_C|GetSpline _splineref))
  (bind _output_get (Variables|Default|SetCurrentPosition (Math|Float|Clamp(Float) (+ (Variables|Default|GetCurrentPosition) (Variables|Default|GetSpeed)) 0.0 (Spline|GetSplineLength (Variables|/Game/Blueprints/FlyingBook/SplineBook.SplineBook_C|GetSpline (Variables|Default|GetSplineRef))))))
  (Transformation|SetActorLocationAndRotation (Spline|GetLocationatDistanceAlongSpline _spline _output_get "World") (Spline|GetRotationatDistanceAlongSpline _spline _output_get "Local")))

(event Custom|Check
  (CallFunction|MoveObject))

(event EventBeginPlay
  (bind _returnvalue (Actor|GetActorOfClass "/Game/Blueprints/FlyingBook/SplineBook.SplineBook_C"))
  (Variables|Default|SetSplineRef _returnvalue))

(event EventTick
  (params (DeltaSeconds :type Float%20%28single-precision%29))
  (for _array_element (Collision|GetOverlappingActors (Variables|Default|GetBox) "/Game/Blueprints/Core/BP_Player.BP_Player_C" :!class /Script/Engine.PrimitiveComponent)
    (bind _asbp_player (Utilities|Casting|CastToBP_Player (Game|GetPlayerCharacter 0)))
    (bind _output_get (Variables|Default|Setbyyyyy (.y (- (Transformation|GetActorLocation _asbp_player) (Transformation|GetActorLocation self)))))
    (if (>= 2e+02 _output_get)
      (Variables|Default|SetSpeed (Variables|Default|GetSpeed_0))
      (elif (>= 5e+02 _output_get)
        (Variables|Default|SetSpeed (Variables|Default|GetSpeed_1))
        (else
          (Variables|Default|SetSpeed (Variables|Default|GetSpeed_2)))))
    (CallFunction|Check)))

(fn ConstructionScript)