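; BP_ControlCheck is a checkpoint trigger that records itself as the player's current respawn point.
; When a BP_Player overlaps its Box, it stores itself as CurrentControlCheck on the BP_MainGameMod game mode.
; Its Respawn function teleports player pawn 0 to the Box's world location, leaving rotation untouched.
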(event OnComponentBeginOverlap(Box)
  (params (OverlappedComponent :type Primitive%20Component%20Object%20Reference) (OtherActor :type Actor%20Object%20Reference) (OtherComp :type Primitive%20Component%20Object%20Reference) (OtherBodyIndex :type Integer) (bFromSweep :type Boolean) (SweepResult :type Hit%20Result%20Structure%20%28by%20ref%29))
  (Utilities|Casting|CastToBP_Player OtherActor)
  (bind _asbp_main_game_mod (Utilities|Casting|CastToBP_MainGameMod (Game|GetGameMode)))
  (Variables|/Game/Blueprints/Core/BP_MainGameMod.BP_MainGameMod_C|SetCurrentControlCheck _asbp_main_game_mod self))

(event EventBeginPlay)

(event Collision|EventActorBeginOverlap
  (params (OtherActor :type Actor%20Object%20Reference)))

(event EventTick
  (params (DeltaSeconds :type Float%20%28single-precision%29)))

(fn ConstructionScript)

(fn Respawn
  (Transformation|SetActorLocation (Game|Player|GetPlayerPawn 0) (Transformation|GetWorldLocation (Variables|Default|GetBox)) false true))