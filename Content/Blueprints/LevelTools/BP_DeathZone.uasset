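; BP_DeathZone is a level trigger that penalizes and repositions BP_Player when it overlaps.
; Each entry in the player's Chars map takes damage equal to a tenth of its MaxHp, with ScreenDamage off for the first entry only.
; Inside that same loop, it calls Respawn on the game mode's CurrentControlCheck, or moves the player to a PlayerStart if none is valid, so repositioning repeats per character.
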(event OnComponentBeginOverlap()
  (params (OverlappedComponent :type Primitive%20Component%20Object%20Reference) (OtherActor :type Actor%20Object%20Reference) (OtherComp :type Primitive%20Component%20Object%20Reference) (OtherBodyIndex :type Integer) (bFromSweep :type Boolean) (SweepResult :type Hit%20Result%20Structure%20%28by%20ref%29))
  (bind _asbp_player (Utilities|Casting|CastToBP_Player OtherActor))
  (bind _values (Utilities|Map|Values (Variables|/Game/Blueprints/Core/BP_Player.BP_Player_C|GetChars _asbp_player)))
  (for (_array_element _array_index) _values
    (Default|TakeDamage _array_element (* (Variables|/Game/Blueprints/DataBase/ParentHeroComponent.ParentHeroComponent_C|GetMaxHp _array_element) 0.1) "NewEnumerator2" (not (== _array_index 0)))
    (bind _asbp_main_game_mod (Utilities|Casting|CastToBP_MainGameMod (Game|GetGameMode)))
    (if (Utilities|IsValid (Variables|/Game/Blueprints/Core/BP_MainGameMod.BP_MainGameMod_C|GetCurrentControlCheck _asbp_main_game_mod))
      (Default|Respawn (Variables|/Game/Blueprints/Core/BP_MainGameMod.BP_MainGameMod_C|GetCurrentControlCheck _asbp_main_game_mod))
      (else
        (bind _returnvalue (Actor|GetActorOfClass "/Script/Engine.PlayerStart"))
        (Transformation|SetActorLocation _asbp_player (Transformation|GetActorLocation _returnvalue) false false)))))

(event EventBeginPlay)

(event Collision|EventActorBeginOverlap
  (params (OtherActor :type Actor%20Object%20Reference)))

(event EventTick
  (params (DeltaSeconds :type Float%20%28single-precision%29)))

(fn ConstructionScript)