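; BP_RotateBlock is a level trigger that turns the player's movement direction and, optionally, the camera.
; A Gate routes either the Interaction event, with an on-screen prompt when IsButtonRotate is set, or the box overlap itself.
; Passing it halves velocity and sets WorldDirection to the Arrow's forward, or to the first-saved player forward if already on the Arrow's axis.
; Two Timelines lerp SpringArm yaw for each case.
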(event OnComponentBeginOverlap(Box)
  (params (OverlappedComponent :type Primitive%20Component%20Object%20Reference) (OtherActor :type Actor%20Object%20Reference) (OtherComp :type Primitive%20Component%20Object%20Reference) (OtherBodyIndex :type Integer) (bFromSweep :type Boolean) (SweepResult :type Hit%20Result%20Structure%20%28by%20ref%29))
  (bind _arrow (Variables|Default|GetArrow))
  (bind _rotateangle (Variables|Default|GetRotateAngle))
  (bind _returnvalue (Math|Vector|GetForwardVector _arrow))
  ;[1 1 1] Подсказка при входе в триггер, если IsButtonRotate True
  (bind _asbp_player (Utilities|Casting|CastToBP_Player OtherActor))
  (if (Variables|Default|GetIsButtonRotate)
    (Widget|SetVisibility (UserInterface|GetWidget (Variables|/Game/Blueprints/Core/BP_Player.BP_Player_C|GetWidget _asbp_player)) "Visible")
    (goto _label Open)
    (else
      (Utilities|FlowControl|Sequence
        (:then_0
          (Utilities|FlowControl|Gate true :!label _label
            (:Exit
              (Variables|/Script/Engine.MovementComponent|SetVelocity (Variables|/Script/Engine.Character|GetCharacterMovement _asbp_player) (* (Pawn|Components|CharacterMovement|GetLastUpdateVelocity (Variables|/Script/Engine.Character|GetCharacterMovement _asbp_player)) 0.5))
              (Utilities|FlowControl|Sequence
                (:then_0
                  (Utilities|FlowControl|DoOnce false
                    (:Completed
                      (Variables|Default|SetLast%20Forward (Transformation|GetActorForwardVector _asbp_player)))))
                (:then_1
                  ;[1 1 1] Поворот камеры игрока
                  (if (Utilities|Operators|EqualEqual (Math|Vector|VectorGetAbs _returnvalue) (Math|Vector|VectorGetAbs (Transformation|GetActorForwardVector _asbp_player)) 0.01)
                    (Variables|/Game/Blueprints/Core/BP_Player.BP_Player_C|SetWorld%20Direction _asbp_player (Variables|Default|GetLast%20Forward))
                    (Variables|Default|SetReturn%20Value%20Z%20%28Yaw%29 (.yaw (Transformation|GetSocketRotation (Variables|/Game/Blueprints/Core/BP_Player.BP_Player_C|GetSpringArm _asbp_player) "None")))
                    (if (Variables|Default|GetIsRotateCamera)
                      (bind _newtrack_0 (Timeline|Timeline_1 PlayFromStart)
                        (:Update
                          (Transformation|SetRelativeRotation (Variables|/Game/Blueprints/Core/BP_Player.BP_Player_C|GetSpringArm _asbp_player) (Math|Rotator|MakeRotator (.roll (Class|SpringArmComponent|GetTargetRotation (Variables|/Game/Blueprints/Core/BP_Player.BP_Player_C|GetSpringArm _asbp_player))) (.pitch (Class|SpringArmComponent|GetTargetRotation (Variables|/Game/Blueprints/Core/BP_Player.BP_Player_C|GetSpringArm _asbp_player))) (Math|Float|Lerp _rotateangle (- _rotateangle (Variables|Default|GetReturn%20Value%20Z%20%28Yaw%29)) _newtrack_0)) false false))))
                    (else
                      (Variables|/Game/Blueprints/Core/BP_Player.BP_Player_C|SetWorld%20Direction _asbp_player _returnvalue)
                      (Variables|Default|SetReturn%20Value%20Z%20%28Yaw%29 (.yaw (Transformation|GetSocketRotation (Variables|/Game/Blueprints/Core/BP_Player.BP_Player_C|GetSpringArm _asbp_player) "None")))
                      (if (Variables|Default|GetIsRotateCamera)
                        (bind _newtrack_0_2 (Timeline|Timeline_0 PlayFromStart)
                          (:Update
                            (Transformation|SetRelativeRotation (Variables|/Game/Blueprints/Core/BP_Player.BP_Player_C|GetSpringArm _asbp_player) (Math|Rotator|MakeRotator (.roll (Class|SpringArmComponent|GetTargetRotation (Variables|/Game/Blueprints/Core/BP_Player.BP_Player_C|GetSpringArm _asbp_player))) (.pitch (Class|SpringArmComponent|GetTargetRotation (Variables|/Game/Blueprints/Core/BP_Player.BP_Player_C|GetSpringArm _asbp_player))) (Math|Float|Lerp (Variables|Default|GetReturn%20Value%20Z%20%28Yaw%29) (+ (Variables|Default|GetReturn%20Value%20Z%20%28Yaw%29) (Variables|Default|GetRotateAngle)) _newtrack_0_2)) false false)))))))))))
        (:then_1
          (goto _label Open))))))

(event OnComponentEndOverlap(Box)
  (params (OverlappedComponent :type Primitive%20Component%20Object%20Reference) (OtherActor :type Actor%20Object%20Reference) (OtherComp :type Primitive%20Component%20Object%20Reference) (OtherBodyIndex :type Integer))
  (bind _arrow (Variables|Default|GetArrow))
  (bind _rotateangle (Variables|Default|GetRotateAngle))
  (bind _returnvalue (Math|Vector|GetForwardVector _arrow))
  ;[1 1 1] Скрытие подсказки при выходе из тригера
  (bind _asbp_player (Utilities|Casting|CastToBP_Player OtherActor))
  (Widget|SetVisibility (UserInterface|GetWidget (Variables|/Game/Blueprints/Core/BP_Player.BP_Player_C|GetWidget _asbp_player)) "Hidden")
  (Utilities|FlowControl|Gate true) ; enters at Close
)

(event OnComponentHit(Box)
  (params (HitComponent :type Primitive%20Component%20Object%20Reference) (OtherActor :type Actor%20Object%20Reference) (OtherComp :type Primitive%20Component%20Object%20Reference) (NormalImpulse :type Vector :default "0, 0, 0") (Hit :type Hit%20Result%20Structure%20%28by%20ref%29))
  (Development|PrintString "Hello"))

(event Custom|CustomEvent
  (params (OverlappedComponent :type Primitive%20Component%20Object%20Reference) (OtherActor :type Actor%20Object%20Reference) (OtherComp :type Primitive%20Component%20Object%20Reference) (OtherBodyIndex :type Integer)))

(event EventBeginPlay)

(event Collision|EventActorBeginOverlap
  (params (OtherActor :type Actor%20Object%20Reference)))

(event EventInteraction
  (bind _arrow (Variables|Default|GetArrow))
  (bind _rotateangle (Variables|Default|GetRotateAngle))
  (bind _returnvalue (Math|Vector|GetForwardVector _arrow))
  (Utilities|FlowControl|Gate true
    (:Exit
      (Variables|/Script/Engine.MovementComponent|SetVelocity (Variables|/Script/Engine.Character|GetCharacterMovement (stale OnComponentBeginOverlap(Box) _asbp_player)) (* (Pawn|Components|CharacterMovement|GetLastUpdateVelocity (Variables|/Script/Engine.Character|GetCharacterMovement (stale OnComponentBeginOverlap(Box) _asbp_player))) 0.5))
      (Utilities|FlowControl|Sequence
        (:then_0
          (Utilities|FlowControl|DoOnce false
            (:Completed
              (Variables|Default|SetLast%20Forward (Transformation|GetActorForwardVector (stale OnComponentBeginOverlap(Box) _asbp_player))))))
        (:then_1
          ;[1 1 1] Поворот камеры игрока
          (if (Utilities|Operators|EqualEqual (Math|Vector|VectorGetAbs _returnvalue) (Math|Vector|VectorGetAbs (Transformation|GetActorForwardVector (stale OnComponentBeginOverlap(Box) _asbp_player))) 0.01)
            (Variables|/Game/Blueprints/Core/BP_Player.BP_Player_C|SetWorld%20Direction (stale OnComponentBeginOverlap(Box) _asbp_player) (Variables|Default|GetLast%20Forward))
            (Variables|Default|SetReturn%20Value%20Z%20%28Yaw%29 (.yaw (Transformation|GetSocketRotation (Variables|/Game/Blueprints/Core/BP_Player.BP_Player_C|GetSpringArm (stale OnComponentBeginOverlap(Box) _asbp_player)) "None")))
            (if (Variables|Default|GetIsRotateCamera)
              (bind _newtrack_0 (Timeline|Timeline_1 PlayFromStart)
                (:Update
                  (Transformation|SetRelativeRotation (Variables|/Game/Blueprints/Core/BP_Player.BP_Player_C|GetSpringArm (stale OnComponentBeginOverlap(Box) _asbp_player)) (Math|Rotator|MakeRotator (.roll (Class|SpringArmComponent|GetTargetRotation (Variables|/Game/Blueprints/Core/BP_Player.BP_Player_C|GetSpringArm (stale OnComponentBeginOverlap(Box) _asbp_player)))) (.pitch (Class|SpringArmComponent|GetTargetRotation (Variables|/Game/Blueprints/Core/BP_Player.BP_Player_C|GetSpringArm (stale OnComponentBeginOverlap(Box) _asbp_player)))) (Math|Float|Lerp _rotateangle (- _rotateangle (Variables|Default|GetReturn%20Value%20Z%20%28Yaw%29)) _newtrack_0)) false false))))
            (else
              (Variables|/Game/Blueprints/Core/BP_Player.BP_Player_C|SetWorld%20Direction (stale OnComponentBeginOverlap(Box) _asbp_player) _returnvalue)
              (Variables|Default|SetReturn%20Value%20Z%20%28Yaw%29 (.yaw (Transformation|GetSocketRotation (Variables|/Game/Blueprints/Core/BP_Player.BP_Player_C|GetSpringArm (stale OnComponentBeginOverlap(Box) _asbp_player)) "None")))
              (if (Variables|Default|GetIsRotateCamera)
                (bind _newtrack_0_2 (Timeline|Timeline_0 PlayFromStart)
                  (:Update
                    (Transformation|SetRelativeRotation (Variables|/Game/Blueprints/Core/BP_Player.BP_Player_C|GetSpringArm (stale OnComponentBeginOverlap(Box) _asbp_player)) (Math|Rotator|MakeRotator (.roll (Class|SpringArmComponent|GetTargetRotation (Variables|/Game/Blueprints/Core/BP_Player.BP_Player_C|GetSpringArm (stale OnComponentBeginOverlap(Box) _asbp_player)))) (.pitch (Class|SpringArmComponent|GetTargetRotation (Variables|/Game/Blueprints/Core/BP_Player.BP_Player_C|GetSpringArm (stale OnComponentBeginOverlap(Box) _asbp_player)))) (Math|Float|Lerp (Variables|Default|GetReturn%20Value%20Z%20%28Yaw%29) (+ (Variables|Default|GetReturn%20Value%20Z%20%28Yaw%29) (Variables|Default|GetRotateAngle)) _newtrack_0_2)) false false)))))))))))

(fn ConstructionScript)