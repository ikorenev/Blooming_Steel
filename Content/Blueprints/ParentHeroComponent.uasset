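; Base hero component that holds combat stats and declares the shared ability functions for heroes.
; Initialization copies stats from row "1" of the Heroes data table and sets current HP to max, while the Energy reset is left unconnected.
; Ultimate spends Energy when it covers UltimateCost.
; SkillAttack, SkillMove, AutoAttack and AddEnergy are empty stubs, and BeginPlay and Tick are unused.
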(event EventBeginPlay)

(event EventTick
  (params (DeltaSeconds :type Float%20%28single-precision%29)))

(fn Initialization
  (bind _returnvalue (Utilities|GetDataTableRow "/Game/Blueprints/DataBase/Heroes.Heroes" "1")
    (:then
      (Utilities|FlowControl|Sequence
        (:then_0
          (bind _output_get (Variables|Default|SetMaxHp (.maxhp _returnvalue)))
          (Variables|Default|SetCurrentHP _output_get))
        (:then_1
          (Variables|Default|SetPhisDef (.phisdef _returnvalue)))
        (:then_2
          (Variables|Default|SetMageDef (.magedef _returnvalue)))
        (:then_3
          (Variables|Default|SetPhisDamage (.phisdamage _returnvalue)))
        (:then_4
          (Variables|Default|SetMageDamage (.magedamage _returnvalue)))
        (:then_5
          (Variables|Default|SetSpeedChar (.speedchar _returnvalue)))
        (:then_6
          (Variables|Default|SetAttackSpeed (.attackspeed _returnvalue)))
        (:then_7
          (Variables|Default|SetCritRate (.critrate _returnvalue)))
        (:then_8
          (Variables|Default|SetCritDamage (.critdamage _returnvalue)))
        (:then_9
          (Variables|Default|SetEnergyRecharge (.energyrecharge _returnvalue)))
        (:then_10
          (Variables|Default|SetTimeSkillCD (.timeskillcd _returnvalue)))
        (:then_11
          (Variables|Default|SetHealPower (.healpower _returnvalue)))
        (:then_12
          (Variables|Default|SetUltimateCost (.ultimatecost _returnvalue)))))))

(fn SkillAttack)

(fn SkillMove)

(fn Ultimate
  (if (>= (Variables|Default|GetEnergy) (Variables|Default|GetUltimateCost))
    (Variables|Default|SetEnergy (- (Variables|Default|GetEnergy) (Variables|Default|GetUltimateCost)))))

(fn AutoAttack)

(fn AddEnergy)