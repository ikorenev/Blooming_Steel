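; BP_Drop is an actor driving a Niagara drop effect that reacts to the player character.
; It feeds a point above the player's mesh into the system every tick and registers itself for exported particle data.
; A particle close to the mesh raises the Force parameter and sets a looping timer, which clears Force and restarts the effect to spawn the drop again.
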(event Custom|SpawnDrop
  (bind _niagara (Variables|Default|GetNiagara))
  (Niagara|SetNiagaraVariable(Float) _niagara "Force" 0.0)
  (Components|Activation|SetActive _niagara true true))

(event EventBeginPlay
  (Class|NiagaraComponent|SetVariableObject (Variables|Default|GetNiagara) "ParticleCallback" self))

(event EventParticleData
  (params (Data :type Array%20of%20Basic%20Particle%20Data%20Structures) (NiagaraSystem :type Niagara%20System%20Object%20Reference) (SimulationPositionOffset :type Vector%20%28by%20ref%29 :default "0, 0, 0"))
  (for _array_element Data
    (if (< (Math|Vector|VectorLength (- (.position _array_element) (Transformation|GetWorldLocation (Variables|/Script/Engine.Character|GetMesh (Game|GetPlayerCharacter 0))))) 5e+01)
      (Niagara|SetNiagaraVariable(Float) (Variables|Default|GetNiagara) "Force" 2.0)
      (Utilities|Time|SetTimerbyFunctionName 0 "SpawnDrop" 5.0 true))))

(event EventTick
  (params (DeltaSeconds :type Float%20%28single-precision%29))
  (Niagara|SetNiagaraVariable(Vector3) (Variables|Default|GetNiagara) "ActorLocation" (+ (Transformation|GetWorldLocation (Variables|/Script/Engine.Character|GetMesh (Game|GetPlayerCharacter 0))) "0.000000,0.000000,150.000000")))

(fn ConstructionScript)