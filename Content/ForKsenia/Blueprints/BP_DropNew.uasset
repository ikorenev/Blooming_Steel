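; BP_DropNew is a drop actor whose Niagara particles track the active player and disappear once one gets close to the player pawn.
; Tick feeds the BP_IzometriaCamera pawn's ActivePlayer location, raised slightly, into the Niagara system.
; The actor receives exported particle positions as the Niagara callback and measures them against the player pawn itself, not ActivePlayer.
; A close particle sets Force and starts a one-second timer on SpawnDrop, which only destroys the actor.
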(event Custom|SpawnDrop
  (Actor|DestroyActor))

(event EventBeginPlay
  (Class|NiagaraComponent|SetVariableObject (Variables|Default|GetNiagara) "ParticleCallback" self))

(event EventTick
  (params (DeltaSeconds :type Float%20%28single-precision%29))
  (bind _asbp_izometria_camera (Utilities|Casting|CastToBP_IzometriaCamera (Game|Player|GetPlayerPawn 0)))
  (Niagara|SetNiagaraVariable(Vector3) (Variables|Default|GetNiagara) "ActorLocation" (+ (Transformation|GetWorldLocation (Variables|/Script/Engine.Actor|GetRootComponent (Variables|/Game/AssetCore/Blueprints/Core/BP_IzometriaCamera.BP_IzometriaCamera_C|GetActivePlayer _asbp_izometria_camera))) "0.000000,0.000000,60.000000")))

(event EventParticleData
  (params (Data :type Array%20of%20Basic%20Particle%20Data%20Structures) (NiagaraSystem :type Niagara%20System%20Object%20Reference) (SimulationPositionOffset :type Vector%20%28by%20ref%29 :default "0, 0, 0"))
  (for _array_element Data
    (if (< (Math|Vector|VectorLength (- (.position _array_element) (Transformation|GetWorldLocation (Variables|/Script/Engine.Actor|GetRootComponent (Game|Player|GetPlayerPawn 0))))) 1e+02)
      (Niagara|SetNiagaraVariable(Float) (Variables|Default|GetNiagara) "Force" 6.0)
      (Utilities|Time|SetTimerbyFunctionName 0 "SpawnDrop" 1.0 true))))

(fn ConstructionScript)