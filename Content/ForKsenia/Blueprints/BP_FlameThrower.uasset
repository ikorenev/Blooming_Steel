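; Flamethrower actor that turns its Sphere component to track the first player's pawn.
; A looping timer set on BeginPlay eases the sphere toward the look-at yaw, with a fixed 90-degree offset, using RInterpTo.
; The interpolation reads DeltaSeconds from the otherwise empty Tick rather than the timer interval.
; The construction script applies a color parameter to the FlameThrowerNS effect.
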(event Custom|Event
  (Transformation|SetWorldRotation (Variables|Default|GetSphere) (Math|Interpolation|RInterpTo (Transformation|GetWorldRotation (Variables|Default|GetSphere)) (Math|Rotator|CombineRotators (Math|Rotator|MakeRotator 0.0 0.0 (.yaw (Math|Rotator|FindLookatRotation (Transformation|GetWorldLocation (Variables|Default|GetSphere)) (Transformation|GetActorLocation (Game|Player|GetPlayerPawn 0))))) "0.000000,-90.000000,0.000000") (stale EventTick DeltaSeconds) (Variables|Default|GetInterp%20Speed)) false false))

(event EventTick
  (params (DeltaSeconds :type Float%20%28single-precision%29)))

(event EventBeginPlay
  (Utilities|Time|SetTimerbyEvent (delegate Custom|Event) 0.05 true))

(fn ConstructionScript
  (Effects|Components|ParticleSystem|SetColorParameter (Variables|Default|GetFlameThrower_NS) (Variables|Default|GetParameter%20Name) (Variables|Default|GetParam)))