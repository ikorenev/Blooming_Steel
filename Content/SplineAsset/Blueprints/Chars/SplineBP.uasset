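; Spline path actor that moves a referenced actor left and right along its curve, driven by the player pawn's MoveLeft and MoveRight events.
; BeginPlay binds both events and derives a constant step from character speed over spline length.
; Each move checks the pawn's block flag, then shifts spline time and sweeps the actor there, keeping pawn height and flipping yaw for left.
; Only leftward movement clamps spline time.
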(event Custom|MoveRight
  (bind _spline (Variables|Default|GetSpline))
  (bind _asbp_side_scroller_character (Utilities|Casting|CastTo (Game|Player|GetPlayerPawn 0)))
  (if (Variables|Default|GetBlocRight _asbp_side_scroller_character)
    (EventDispatchers|BindEventtoMoveRight (stale EventBeginPlay _asbp_side_scroller_character) (delegate Custom|MoveRight))
    (else
      (Variables|Default|SetTimeSpline (+ (Variables|Default|GetTimeSpline) (Variables|Default|GetMoveForTiick)))
      (Transformation|SetActorTransform (Variables|Default|GetActor%20Reference) (Math|Transform|MakeTransform (Math|Vector|MakeVector (.x (Spline|GetLocationatTime _spline (Variables|Default|GetTimeSpline) "World" true)) (.y (Spline|GetLocationatTime _spline (Variables|Default|GetTimeSpline) "World" true)) (.z (Transformation|GetActorLocation (Game|Player|GetPlayerPawn 0)))) (Class|SplineComponent|GetRotationatTime _spline (Variables|Default|GetTimeSpline) "World" true) "1.000000,1.000000,1.000000") true))))

(event Custom|MoveLeft
  (bind _spline (Variables|Default|GetSpline))
  (bind _asbp_side_scroller_character (Utilities|Casting|CastTo (Game|Player|GetPlayerPawn 0)))
  (if (Variables|Default|GetBlockLeft _asbp_side_scroller_character)
    (EventDispatchers|BindEventtoMoveLeft (stale EventBeginPlay _asbp_side_scroller_character) (delegate Custom|MoveLeft))
    (else
      (Variables|Default|SetTimeSpline (Math|Float|Clamp(Float) (- (Variables|Default|GetTimeSpline) (Variables|Default|GetMoveForTiick))))
      (Transformation|SetActorTransform (Variables|Default|GetActor%20Reference) (Math|Transform|MakeTransform (Math|Vector|MakeVector (.x (Spline|GetLocationatTime _spline (Variables|Default|GetTimeSpline) "World" true)) (.y (Spline|GetLocationatTime _spline (Variables|Default|GetTimeSpline) "World" true)) (.z (Transformation|GetActorLocation (Game|Player|GetPlayerPawn 0)))) (Math|Rotator|MakeRotator (.Roll (Math|Rotator|BreakRotator (Class|SplineComponent|GetRotationatTime _spline (Variables|Default|GetTimeSpline) "World" true))) (.Pitch (Math|Rotator|BreakRotator (Class|SplineComponent|GetRotationatTime _spline (Variables|Default|GetTimeSpline) "World" true))) (- (.Yaw (Math|Rotator|BreakRotator (Class|SplineComponent|GetRotationatTime _spline (Variables|Default|GetTimeSpline) "World" true))) 1.8e+02)) "1.000000,1.000000,1.000000") true))))

(event EventBeginPlay
  (Variables|Default|SetLenghtSpline (Spline|GetSplineLength (Variables|Default|GetSpline)))
  (Variables|Default|SetMoveForTiick (/ (Variables|Default|GetSpeed%20character) (Variables|Default|GetLenghtSpline)))
  (bind _asbp_side_scroller_character (Utilities|Casting|CastTo (Game|Player|GetPlayerPawn 0)))
  (Utilities|FlowControl|Sequence
    (:then_0
      (EventDispatchers|BindEventtoMoveLeft _asbp_side_scroller_character (delegate Custom|MoveLeft)))
    (:then_1
      (EventDispatchers|BindEventtoMoveRight _asbp_side_scroller_character (delegate Custom|MoveRight)))))

(event Collision|EventActorBeginOverlap
  (params (OtherActor :type Actor%20Object%20Reference)))

(event EventTick
  (params (DeltaSeconds :type Float%20%28single-precision%29)))

(fn ConstructionScript)